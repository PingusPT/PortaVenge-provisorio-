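; Player character for what appears to be a stealth game, with coin throw, knife kill and portal kill abilities.
; Coin aiming traces from the cursor, predicts the arc with spawned trajectory actors and places a sound-range marker, walking closer if out of range.
; Knife kill sphere-traces for enemies, aligns both characters and plays paired montages.
; Tick rebuilds a navigation-path spline, though its mesh building and click targeting are disconnected.
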(event `self.ReceiveBeginPlay`
  (bind _bp_fadeobjectscomp (`self.BP_FadeObjectsComp`))
  (`PrimitiveComponent.SetCollisionResponseToChannel` (`self.Mesh`) "ECC_Camera" "ECR_Ignore")
  (set `self.PrevieTargetLocation` (`self.K2_GetActorLocation`))
  (set `self.CanTakeDown` false)
  (`SceneComponent.K2_SetWorldRotation` :`self` (`self.CoinSoundRange`))
  (`SceneComponent.SetHiddenInGame` (`self.CoinSoundRange`) true false)
  (bind _asmain_game_mode (cast `/Game/Bp/Main_GameMode` (`GameplayStatics.GetGameMode`)))
  (set `self.As Main Game Mode` _asmain_game_mode)
  (`LineOfSightComponent.StartLineTrace` (`self.CoinRange`) "TraceTypeQuery9" 60)
  (`LineOfSightComponent.StartBuildMesh` (`self.CoinRange`))
  (`SceneComponent.SetHiddenInGame` (`self.CoinRange`) true false)
  (bind _outactors (`GameplayStatics.GetAllActorsOfClass` "/Game/ParedeSpawnPortal/BP_InvisibleWall.BP_InvisibleWall_C"))
  (set `AdvancedFadeObjectsComponent.actorsIgnore` _outactors _bp_fadeobjectscomp)
  (bind _outactors_2 (`GameplayStatics.GetAllActorsOfClass` "/Game/Bps_Teste/Bp_PortalRef.Bp_PortalRef_C"))
  (set `AdvancedFadeObjectsComponent.actorsIgnore` _outactors_2 _bp_fadeobjectscomp))

(event `ShowPath`
  (params (GoingToAtack :type Boolean) (TargetLocation :type "Vector Structure") (Enemy :type "Actor Object Reference"))
  ;[1 1 1] On Click Set Final Spline Point
)

(event `Throw Coin`
  (bind (_returnvalue_roll _returnvalue_pitch _returnvalue_yaw) (`KismetMathLibrary.BreakRotator` (`KismetMathLibrary.FindLookAtRotation` (`self.K2_GetActorLocation`) (+ (`self.CoinVelocityDirection`) (`self.K2_GetActorLocation`)))))
  (if (`self.CoinAbilityActive=`)
    (`|ExecutionSequence`
      (:`then_0`
        (`/Engine/EditorBlueprintResources/StandardMacros.DoOnce` false :!label _label
          (:`Completed`
            (if (not (`self.InCoinRange`))
              (`|AIMoveTo` self (`KismetMathLibrary.MakeVector` (.x (`self.OutRangeCoin`)) (.y (`self.OutRangeCoin`))) null 1000.0
                (:`OnSuccess`
                  _)))
            (bind _returnvalue (`|SpawnActorFromClass` "/Game/Bps_Teste/Bp_Coin.Bp_Coin_C" (`KismetMathLibrary.MakeTransform` (`self.K2_GetActorLocation`) (`self.K2_GetActorRotation` (`GameplayStatics.GetPlayerPawn` 0)) (0.2 0.2 0.2)) "AlwaysSpawn" "MultiplyWithRoot" null null))
            (set `self.Coin` _returnvalue)
            (`FMODAudioComponent.Play` (`self.TrhowCoin`))
            (`self.K2_SetActorRotation` (`KismetMathLibrary.MakeRotator` _returnvalue_roll 0.0 _returnvalue_yaw))
            (`self.PlayAnimMontage` "/Game/Player_X1/Poses/X1_Coin_Trhow_Montage.X1_Coin_Trhow_Montage")
            (`PrimitiveComponent.SetPhysicsLinearVelocity` (`/Game/Bps_Teste/Bp_Coin.Sphere` (`self.Coin`)) (`self.CoinVelocityDirection`) true "None")
            (set `self.CoinAbilityActive=` false)
            (`SceneComponent.K2_SetWorldLocation` (`self.CoinSoundRange`) (`KismetMathLibrary.MakeVector` (.x (+ (`self.CoinVelocityDirection`) (`self.K2_GetActorLocation`))) (.y (+ (`self.CoinVelocityDirection`) (`self.K2_GetActorLocation`))) 10.0) true false)
            (`/Game/Bp/Bp_CameraController.Change To DefaultAbility` (`/Game/Bp/Main_GameMode.PlayerController` (`self.As Main Game Mode`)))
            (`KismetSystemLibrary.DrawDebugBox` (0.0 0.0 0.0) (30.0 30.0 30.0) (struct :`R` 1.0 :`B` 0.747519 :`A` 1.0) (struct) 30.0 10.0))))
      (:`then_1`
        (`KismetSystemLibrary.Delay` 2.0)
        (goto _label :!via `Reset`)))))

(event `self.ReceiveTick`
  (params (DeltaSeconds :type "Float (single-precision)"))
  (bind (_returnvalue_roll _returnvalue_pitch _returnvalue_yaw) (`KismetMathLibrary.BreakRotator` (`self.K2_GetActorRotation`)))
  (bind _returnvalue (`self.K2_GetActorLocation`))
  (bind _spline (`self.Spline`))
  (bind _spline_2 (`self.Spline`))
  (`|ExecutionSequence`
    (:`then_0`
      ;[1 1 1] If The Player is near of the end of the Spline
      (if (== (`self.PrevieTargetLocation`) (`self.K2_GetActorLocation`) :`ErrorTolerance` 91.9)
        ;[1 1 1] Clear Spline
        (`SplineComponent.ClearSplinePoints` (`self.Spline`) true)
        (set `self.PrevieTargetLocation` (`self.K2_GetActorLocation`))
        (`self.AddSplineMeshes`)
        (else
          ;[1 1 1] Going To atack
          (if (`self.Going to Atack`)
            ;[1 1 1] Build Spline
            (bind _returnvalue_2 (`NavigationSystemV1.FindPathToLocationSynchronously` (`self.K2_GetActorLocation` (`self.Enemy`)) _returnvalue null null))
            (`SplineComponent.ClearSplinePoints` _spline true)
            (for _array_element (`NavigationPath.PathPoints` _returnvalue_2)
              (`SplineComponent.AddSplinePoint` _spline (+ _array_element (0.0 30.0 30.0)) "World" true))
            (else
              (bind _returnvalue_3 (`NavigationSystemV1.FindPathToLocationSynchronously` _returnvalue (`self.PrevieTargetLocation`) null null))
              (`SplineComponent.ClearSplinePoints` _spline_2 true)
              (for _array_element_2 (`NavigationPath.PathPoints` _returnvalue_3)
                (`SplineComponent.AddSplinePoint` _spline_2 (+ _array_element_2 (0.0 30.0 30.0)) "World" true))))
          (`self.AddSplineMeshes`
            (:`Completed`
              (`SceneComponent.SetMobility` (`self.CapsuleComponent`) "Movable"))))))
    (:`then_1`
      (if (`self.CoinAbilityActive=`)
        (`self.MoveCoinRange`)))
    (:`then_2`
      (if (`self.SeeEnemyInCoinRange`)
        _))
    (:`then_3`
      (`self.K2_SetActorRotation` (`KismetMathLibrary.MakeRotator` 0.0 0.0 _returnvalue_yaw)))))

(event `Ativate Coin Ability`
  (bind _coulddowncoin (`/Game/Bp/Rts_Camera.CouldDownCoin` (`/Game/Bp/Main_GameMode.As Rts Camera` (`self.As Main Game Mode`))))
  ;[0 0 0] Activate and deactivate coin visual
  (if (<= _coulddowncoin 0.0)
    (set `self.CoinAbilityActive=` true)
    (`SceneComponent.SetHiddenInGame` (`self.CoinSoundRange`) false false)
    (`SceneComponent.SetHiddenInGame` (`self.CoinRange`) false false)
    (else
      (`KismetSystemLibrary.K2_SetTimerDelegate` (delegate `Ativate Coin Ability`) _coulddowncoin))))

(event `MoveCoinRange`
  (bind (_worldlocation _worlddirection) (`PlayerController.DeprojectMousePositionToWorld` (`GameplayStatics.GetPlayerController` 0)))
  (bind (_outhit _returnvalue) (`KismetSystemLibrary.LineTraceSingle` :`Start` _worldlocation :`End` (+ _worldlocation (* _worlddirection 100000.0)) :`TraceChannel` "TraceTypeQuery5" :`DrawDebugType` "ForDuration" :`DrawTime` 1.0))
  (if _returnvalue
    (bind (_bblockinghit _binitialoverlap _time _distance _location) (`GameplayStatics.BreakHitResult` _outhit))
    (bind _returnvalue_2 (- _location (`self.K2_GetActorLocation`)))
    (if (not (or (> (.x _returnvalue_2) 1000.0) (> (.y _returnvalue_2) 1000.0)))
      ;[1 1 1] Sem Andar
      (set `self.InCoinRange` true)
      (else
        ;[1 1 1] Tem de andar ate ao local
        (set `self.InCoinRange` false)
        (set `self.OutRangeCoin` _location)))
    (set `self.CoinVelocityDirection` (`KismetMathLibrary.MakeVector` (.x (`KismetMathLibrary.ClampVectorSize` _returnvalue_2 0.0 1000.0)) (.y (`KismetMathLibrary.ClampVectorSize` _returnvalue_2 0.0 1000.0)) 10.0))
    (set `self.CoinVelocityDirection` (+ (`self.CoinVelocityDirection`) (0.0 0.0 400.0)))
    (bind _predictresult (`GameplayStatics.Blueprint_PredictProjectilePath_Advanced` (make `PredictProjectilePathParams` (`self.K2_GetActorLocation`) (* (`self.CoinVelocityDirection`) 1.0) true 0.0 1.3 true "ECC_GameTraceChannel10")))
    (bind (_bblockinghit_2 _binitialoverlap_2 _time_2 _distance_2 _location_2 _impactpoint _normal _impactnormal _physmat _hitactor) (`GameplayStatics.BreakHitResult` (`.HitResult` (break `PredictProjectilePathResult` _predictresult))))
    (`/Engine/EditorBlueprintResources/StandardMacros.IsValid` _hitactor
      (:`Is Valid`
        (if (`self.ActorHasTag` _hitactor "Floor")
          (`SceneComponent.K2_SetWorldLocation` (`self.CoinSoundRange`) (`KismetMathLibrary.MakeVector` (.x _location_2) (.y _location_2) (+ (.z _location_2) 30.0)) true false :!label _label_2)
          (`SceneComponent.K2_SetWorldRotation` (`self.CoinSoundRange`) (`self.K2_GetActorRotation` (`GameplayStatics.GetPlayerPawn` 0)) false false)
          (for _array_element (break `PredictProjectilePathResult` _predictresult)
            (`|SpawnActorFromClass` "/Game/Bps_Teste/TrajectoryBp.TrajectoryBp_C" (`KismetMathLibrary.MakeTransform` (break `PredictProjectilePathPointData` _array_element) (`KismetMathLibrary.FindLookAtRotation` (`self.K2_GetActorLocation`) (`SceneComponent.K2_GetComponentLocation` (`self.CoinSoundRange`)))) "AlwaysSpawn" "MultiplyWithRoot" null null))
          (else
            (`SceneComponent.K2_SetWorldLocation` (`self.CoinSoundRange`) (`KismetMathLibrary.MakeVector` (.x _impactpoint) (.y _impactpoint) 30.0) true false)
            (bind (_returnvalue_x _returnvalue_y) (`KismetMathLibrary.BreakVector` (- (`KismetMathLibrary.MakeVector` (.x _impactpoint) (.y _impactpoint)) (`self.K2_GetActorLocation`))))
            (set `self.CoinVelocityDirection` (`KismetMathLibrary.MakeVector` _returnvalue_x _returnvalue_y 400.0))
            (bind _predictresult_2 (`GameplayStatics.Blueprint_PredictProjectilePath_Advanced` (make `PredictProjectilePathParams` (`self.K2_GetActorLocation`) (* (`self.CoinVelocityDirection`) 1.0) true 0.0 1.3 true "ECC_GameTraceChannel10")))
            (for _array_element_2 (break `PredictProjectilePathResult` _predictresult_2)
              (`|SpawnActorFromClass` "/Game/Bps_Teste/TrajectoryBp.TrajectoryBp_C" (`KismetMathLibrary.MakeTransform` (break `PredictProjectilePathPointData` _array_element_2) (`KismetMathLibrary.FindLookAtRotation` (`self.K2_GetActorLocation`) (`SceneComponent.K2_GetComponentLocation` (`self.CoinSoundRange`)))) "AlwaysSpawn" "MultiplyWithRoot" null null)))))
      (:`Is Not Valid`
        (goto _label_2)))))

(event `KilledTheEnemy`
  (set `self.Going to Atack` false)
  (set `self.Enemy` null)
  (set `self.PrevieTargetLocation` (`self.K2_GetActorLocation`)))

(event `UpdateReverbFootStep`
  (params (reverb :type "Float (double-precision)"))
  (`FMODAudioComponent.SetParameter` (`self.FMODAudio`) "Reverb" reverb))

(event `DeActivate Coin Ability`
  (set `self.CoinAbilityActive=` false)
  (`SceneComponent.SetHiddenInGame` (`self.CoinSoundRange`) true false)
  (`SceneComponent.SetHiddenInGame` (`self.CoinRange`) true false))

(event `PlayFootStep`
  (`FMODAudioComponent.Play` (`self.FMODAudio`)))

(event `PortalKill`
  (`self.PlayAnimMontage` "/Game/Player_X1/Poses/X1_PortalKill_Montage.X1_PortalKill_Montage")
  (`FMODAudioComponent.Play` (`self.PortalSound`))
  (`NiagaraFunctionLibrary.SpawnSystemAtLocation` "/Game/StarterContent/Maps/CaixaDeAreiaVFXs/Portal/NS_Portal3.NS_Portal3" (+ (- (`self.K2_GetActorLocation`) (0.0 0.0 50.0)) (+ (* (`self.GetActorForwardVector`) 50.0) (* (`self.GetActorRightVector`) 50.0))) (`KismetMathLibrary.MakeRotator` (.roll (`self.K2_GetActorRotation`)) 90.0 (.yaw (`self.K2_GetActorRotation`)))))

(event `KnifeKill`
  (bind _returnvalue (`self.K2_GetActorLocation`))
  (bind (_returnvalue_roll _returnvalue_pitch _returnvalue_yaw) (`KismetMathLibrary.BreakRotator` (`KismetMathLibrary.FindLookAtRotation` (`self.K2_GetActorLocation`) (`self.K2_GetActorLocation` (`self.TargetKill`)))))
  (bind (_outhit _returnvalue_2) (`KismetSystemLibrary.SphereTraceSingle` _returnvalue _returnvalue 300.0 "TraceTypeQuery11" false (`|MakeArray` (`GameplayStatics.GetPlayerPawn` 0) :!type "Actor Object Reference")))
  (if _returnvalue_2
    (bind (_bblockinghit _binitialoverlap _time _distance _location _impactpoint _normal _impactnormal _physmat _hitactor) (`GameplayStatics.BreakHitResult` _outhit))
    (if (`self.ActorHasTag` _hitactor "Enemy")
      (`FMODAudioComponent.Play` (`self.KillKnife`))
      (bind _ascharacter (cast `Character` _hitactor))
      (set `self.TargetKill` _ascharacter)
      (bind _asbp_ai_enemy (cast `/Game/AI/Bp_AiEnemy` _ascharacter)
        (:`then`
          (set `/Game/AI/Bp_AiEnemy.Patroling?` false _asbp_ai_enemy))
        (:`CastFailed`
          _))
      (`|AIMoveTo` (`self.TargetKill`) (`SceneComponent.K2_GetComponentLocation` (`self.AnimationRef`)) null 10000.0
        (:`OnSuccess`
          (`self.K2_SetActorRotation` (`self.TargetKill`) (`SceneComponent.K2_GetComponentRotation` (`self.AnimationRef`)) false)
          (`self.K2_SetActorRotation` (`KismetMathLibrary.MakeRotator` 0.0 0.0 _returnvalue_yaw))
          (bind _asbp_v2ai_controller (cast `/Game/AI/Bp_V2AiController` (`self.GetController` (`self.TargetKill`))))
          (`/Game/AI/Bp_V2AiController.DestroiVisiom` _asbp_v2ai_controller)
          (bind _asbp_ai_enemy_2 (cast `/Game/AI/Bp_AiEnemy` (`self.TargetKill`))
            (:`then`
              (bind _returnvalue_3 (`self.PlayAnimMontage` _asbp_ai_enemy_2 "/Game/Inimigos/Pequeno/ANIM/Knife_Dead_Montage.Knife_Dead_Montage" 1.0 "None"))
              (`KismetSystemLibrary.K2_SetTimerDelegate` (delegate `DisableMovement`) (- _returnvalue_3 0.5))
              (`self.PlayAnimMontage` self "/Game/Player_X1/Poses/X1_KnifeKill_Montage.X1_KnifeKill_Montage" 1.0 "None"))
            (:`CastFailed`
              (bind _returnvalue_4 (`self.PlayAnimMontage` (`self.TargetKill`) "/Game/Inimigos/Gordo/ANIM/IG_DeathAnim_Montage.IG_DeathAnim_Montage" 1.0 "None"))
              (`KismetSystemLibrary.K2_SetTimerDelegate` (delegate `DisableMovement`) (- _returnvalue_4 0.5))
              (`self.PlayAnimMontage` self "/Game/Player_X1/Poses/X1_KnifeIGKill_Montage.X1_KnifeIGKill_Montage" 1.0 "None")))
          (`KismetSystemLibrary.Delay` 1.3)
          (`/Game/AI/Bp_V2AiController.PlaySound Death` _asbp_v2ai_controller))))))

(event `DisableMovement`
  (message `/Game/Interfaces/RaggdollKill.Kill Actor` (`self.TargetKill`)))

(event `self.CoinSoundRange.OnComponentBeginOverlap`
  (params (OverlappedComponent :type "PrimitiveComponent Object Reference") (OtherActor :type "Actor Object Reference") (OtherComp :type "PrimitiveComponent Object Reference") (OtherBodyIndex :type Integer) (bFromSweep :type Boolean) (SweepResult :type "HitResult Structure (by ref)"))
  (if (`self.ActorHasTag` OtherActor "Enemy")
    (set `self.EnemyInCoinRange` true)
    (set `self.EnemyInCoinRang` OtherActor)))

(event `self.CoinSoundRange.OnComponentEndOverlap`
  (params (OverlappedComponent :type "PrimitiveComponent Object Reference") (OtherActor :type "Actor Object Reference") (OtherComp :type "PrimitiveComponent Object Reference") (OtherBodyIndex :type Integer))
  (if (`self.ActorHasTag` OtherActor "Enemy")
    (set `self.EnemyInCoinRange` true)
    (set `self.EnemyInCoinRang` null)))

(fn `UserConstructionScript`)