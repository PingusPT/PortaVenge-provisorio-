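; Hackable security camera that sweeps on a timeline and catches actors tagged Detectable entering its view cone.
; Cone overlap plays a detection sound and triggers the player controller's death widget, while a Tick line trace confirms sight and turns the camera toward the player.
; Clicking starts a hack through the player controller, tied to a Snake minigame widget.
; When not working, it restarts after ten seconds; stopped cameras begin hidden until Ligar reveals them.
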(event `Ligar`
  (`KismetSystemLibrary.Delay` (`KismetMathLibrary.RandomFloatInRange` 0.0 0.5))
  (`self.SetActorHiddenInGame` false)
  (`SceneComponent.SetHiddenInGame` (`self.StaticMesh`) false false)
  (`SceneComponent.SetHiddenInGame` (`self.Cone`) false false))

(event `self.ReceiveBeginPlay`
  (bind _playercontroller (`/Game/Bp/Main_GameMode.PlayerController` (`self.As Main Game Mode`)))
  (`FMODAudioComponent.Play` (`self.CameraRoda`))
  (`FMODAudioComponent.Stop` (`self.MusicaMiniGame`))
  (`FMODAudioComponent.Stop` (`self.FMODDetect`))
  (if (`self.StopedCamera`)
    (`self.SetActorHiddenInGame` true)
    (`SceneComponent.SetHiddenInGame` (`self.StaticMesh`) true false)
    (`SceneComponent.SetHiddenInGame` (`self.Cone`) true false)
    (else
      (`self.CamaraRotation`)))
  (set `self.InitialRotator` (`SceneComponent.GetSocketRotation` (`self.DefaultSceneRoot`) "None"))
  (set `self.CameraWorking` true)
  (`KismetSystemLibrary.Delay` 1.0)
  (bind _asmain_game_mode (cast `/Game/Bp/Main_GameMode` (`GameplayStatics.GetGameMode`)))
  (set `self.As Main Game Mode` _asmain_game_mode)
  (set `self.Player` (`/Game/Bp/Main_GameMode.Player` (`self.As Main Game Mode`)))
  (bind _returnvalue (`GameplayStatics.GetActorOfClass` "/Game/Bp/SnakeMiniGame.SnakeMiniGame_C"))
  (bind _assnake_mini_game (cast `/Game/Bp/SnakeMiniGame` _returnvalue))
  (set `self.As Snake Mini Game` _assnake_mini_game)
  (set `self.SnakeSpawn` (`SceneComponent.GetChildComponent` (`/Game/Bp/SnakeMiniGame.DefaultSceneRoot` _assnake_mini_game) 1))
  (set `PlayerController.bEnableClickEvents` true _playercontroller)
  (set `PlayerController.bEnableClickEvents` true _playercontroller))

(event `self.Cone.OnComponentBeginOverlap`
  (params (OverlappedComponent :type "PrimitiveComponent Object Reference") (OtherActor :type "Actor Object Reference") (OtherComp :type "PrimitiveComponent Object Reference") (OtherBodyIndex :type Integer) (bFromSweep :type Boolean) (SweepResult :type "HitResult Structure (by ref)"))
  ;[1 1 1] On Begin See Player
  (if (and (`self.ActorHasTag` OtherActor "Detectable") (`self.CameraWorking`))
    (set `self.DetectedActor` OtherActor)
    (set `self.IsInArea` true)
    (`FMODAudioComponent.Play` (`self.FMODDetect`))
    (`ActorComponent.Activate` (`self.DetectionExclamatione`) false)
    (`/Engine/EditorBlueprintResources/StandardMacros.DoOnce` false
      (:`Completed`
        (`/Game/Bp/Bp_CameraController.DeathWidget` (`/Game/Bp/Main_GameMode.PlayerController` (`self.As Main Game Mode`)))))))

(event `self.Cone.OnComponentEndOverlap`
  (params (OverlappedComponent :type "PrimitiveComponent Object Reference") (OtherActor :type "Actor Object Reference") (OtherComp :type "PrimitiveComponent Object Reference") (OtherBodyIndex :type Integer))
  ;[1 1 1] On End See Character
  (cast `/Game/Bp/Bp_Character` OtherActor)
  (set `self.IsInArea` false))

(event `self.ReceiveTick`
  (params (DeltaSeconds :type "Float (single-precision)"))
  ;[1 1 1] Camara Working
  (if (`self.CameraWorking`)
    (if (`self.IsInArea`)
      (`self.TraceCheck`
        (:`true`
          (`self.StopRotation`)
          (`self.Rotate`))))
    (else
      (`self.StopRotation`)
      (`FMODAudioComponent.Stop` (`self.CameraRoda`))
      (`KismetSystemLibrary.Delay` 10.0)
      (set `self.CameraWorking` true)
      (`self.ActivateCamera` false)
      (`self.CamaraRotation`)
      (set `self.CameraIsOff` false)
      (`FMODAudioComponent.Play` (`self.CameraRoda`)))))

(event `CamaraRotation`
  ;[1 1 1] Camara Rotation
  (if (`self.RotateInverse`)
    (bind (_direction _newtrack_0) (`Timeline|RotateCamera` :!label _label)
      (:`Update`
        (`SceneComponent.K2_SetRelativeRotation` (`self.StaticMesh`) (`KismetMathLibrary.MakeRotator` (.roll (`self.InitialRotator`)) (.pitch (`self.InitialRotator`)) (+ (* _newtrack_0 (`self.RotationDegrees`)) (.yaw (`self.InitialRotator`)))) false false))
      (:`Finished`
        (set `self.RotateInverse` (not (`self.RotateInverse`)))
        (`self.CamaraRotation`)))
    (else
      (goto _label :!via `Reverse`))))

(event `StopRotation`
  ;[1 1 1] Camara Rotation
  (goto _label :!via `Stop`))

(event `/Game/Bp/Hackable.Hack`
  (params (Camera :type "CameraComponent Object Reference")))

(event `EnableSpawks`
  (`ActorComponent.Activate` (`self.Spark_NS`) false)
  (`KismetSystemLibrary.Delay` 10.0)
  (`ActorComponent.Deactivate` (`self.Spark_NS`)))

(event `EnableOverlay`)

(event `Camera_Off`
  (`ActorComponent.SetActive` (`self.Cone`) false false)
  (set `self.CameraIsOff` true)
  (set `self.CameraWorking` true))

(event `ResetWidget`
  (`FMODAudioComponent.Stop` (`self.MusicaMiniGame`))
  (goto _label_2 :!via `Reset`))

(event `Click On Camera`
  (bind _snakewidget (`self.SnakeWidget`))
  (if (not (`self.CameraIsOff`))
    (`FMODAudioComponent.Play` (`self.MusicaMiniGame`))
    (`FMODAudioComponent.Play` (`self.ActivateHack`))
    (`|ExecutionSequence`
      (:`then_0`
        (`/Engine/EditorBlueprintResources/StandardMacros.DoOnce` false :!label _label_2
          (:`Completed`
            (bind _returnvalue (`|CreateWidget` "/Game/Widgets/Snake/Snake_Minigame_Widget.Snake_Minigame_Widget_C" (`/Game/Bp/Main_GameMode.PlayerController` (`self.As Main Game Mode`))))
            (set `self.SnakeWidget` _returnvalue)
            (`UserWidget.AddToViewport` _returnvalue 0))))
      (:`then_1`
        (`/Engine/EditorBlueprintResources/StandardMacros.IsValid` _snakewidget
          (:`Is Valid`
            (message `/Game/Interfaces/SparklCam.Sparkle` (`/Game/Bp/Main_GameMode.PlayerController` (`self.As Main Game Mode`)) self _snakewidget)
            (`/Game/Bp/Bp_CameraController.CameraHack` (`/Game/Bp/Main_GameMode.PlayerController` (`self.As Main Game Mode`)))))))))

(event `self.StaticMesh.OnClicked`
  (params (TouchedComponent :type "PrimitiveComponent Object Reference") (ButtonPressed :type "Key Structure")))

(fn `ActivateCamera`
  (params (active :type Boolean))
  (bind _returnvalue (not active))
  (set `self.CameraWorking` _returnvalue)
  (`SceneComponent.SetVisibility` (`self.Cone`) _returnvalue false)
  (`SceneComponent.SetVisibility` (`self.SpotLight`) _returnvalue false))

(fn `UserConstructionScript`)