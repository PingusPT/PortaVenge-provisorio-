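; Test actor for procedural line-of-sight mesh generation.
; On BeginPlay its LineOfSight component starts 60 Visibility line traces and builds a mesh; Tick draws a debug sphere sized from that component's bounds.
; An older prototype remains disconnected: forward, left and right Arrow traces feeding BuildMesh, which makes a single ProceduralMesh triangle from the hit points.
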(event `self.ReceiveBeginPlay`
  (`LineOfSightComponent.StartLineTrace` (`self.LineOfSight`) "TraceTypeQuery1" 60)
  (`LineOfSightComponent.StartBuildMesh` (`self.LineOfSight`)))

(event `self.ReceiveTick`
  (params (DeltaSeconds :type "Float (single-precision)"))
  (bind (_origin _boxextent) (`KismetSystemLibrary.GetComponentBounds` (`self.LineOfSight`)))
  (`KismetSystemLibrary.DrawDebugSphere` (`self.K2_GetActorLocation`) (/ (+ (.x _boxextent) (.y _boxextent)) 2.0) 12 (struct :`R` 0.936309 :`B` 1.0 :`A` 1.0) 0.1 10.0))

(fn `BuildMesh`
  (bind _rightlocation (`self.RightLocation`))
  (`KismetSystemLibrary.DrawDebugBox` _rightlocation (10.0 10.0 10.0) (struct :`R` 0.210826 :`G` 1.0 :`B` 0.298002 :`A` 1.0) (struct) 0.1 10.0)
  (`ProceduralMeshComponent.CreateMeshSection_LinearColor` :`self` (`self.ProceduralMesh`) :`Vertices` (`|MakeArray` (- (`self.LeftLocation`) (`self.K2_GetActorLocation`)) (- (`self.LocationForward`) (`self.K2_GetActorLocation`)) (- _rightlocation (`self.K2_GetActorLocation`))) :`Triangles` (`|MakeArray` 2 1 0)))

(fn `UserConstructionScript`)