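; Portal arm actor that grabs an enemy and pulls back toward its portal.
; HandGrab moves the passed Portal actor 100 units behind the arm's axis-aligned facing, then homes ProjectileMovement on the enemy's "Pivot" component and back to that point.
; Overlapping an "Enemy" Character sets the target, physics-constrains its left shoulder to the arm's Cube, then kills and destroys it after a delay.
; Debug prints, boxes and an unused MoveComponentTo approach remain.
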(event `DeLadoComFrenteADireita`
  ;[1 1 1] Definir ponto de Saida
  (bind _output_get (set `self.BeginPosition` (`KismetMathLibrary.MakeVector` (.x (`SceneComponent.K2_GetComponentLocation` (`self.Cube`))) (- (.y (`SceneComponent.K2_GetComponentLocation` (`self.Cube`))) 100.0) (.z (`SceneComponent.K2_GetComponentLocation` (`self.Cube`))))))
  (`KismetSystemLibrary.DrawDebugBox` _output_get (10.0 10.0 10.0) (struct :`R` 0.128808 :`G` 0.976124 :`B` 1.0 :`A` 1.0) (struct) 1000.0)
  (`self.K2_SetActorLocation` (`self.AimPoint`) _output_get false true)
  (`self.Move`))

(event `HandGrab`
  (params (Portal :type "/Game/Bp/Bp_AimPoint Object Reference"))
  (bind _returnvalue (`self.GetActorForwardVector` self))
  (set `self.AimPoint` Portal)
  (set `self.FoardVector` _returnvalue)
  (if (or (== _returnvalue (1.0 0.0 0.0) :`ErrorTolerance` 0.1) (== _returnvalue (-1.0 0.0 0.0) :`ErrorTolerance` 0.1))
    ;[1 1 1] Que lado esta do eixo Y
    (`KismetSystemLibrary.PrintString` "Frente")
    (if (== (`self.FoardVector`) (1.0 0.0 0.0) :`ErrorTolerance` 0.1)
      (`KismetSystemLibrary.PrintString` "Direita" true true (struct :`R` 1.0 :`G` 0.514237 :`A` 1.0) 10.0)
      (`self.DeFrenteComFrenteADireita`)
      (else
        (`KismetSystemLibrary.PrintString` "Esquerda" true true (struct :`R` 1.0 :`B` 0.181547 :`A` 1.0) 10.0)
        (`self.DeFrenteComFrenteAEsquerda`)))
    (else
      (`KismetSystemLibrary.PrintString` "Lado")
      (if (== (`self.FoardVector`) (0.0 1.0 0.0) :`ErrorTolerance` 0.1)
        (`KismetSystemLibrary.PrintString` "Direita" true true (struct :`R` 1.0 :`G` 0.514237 :`A` 1.0) 10.0)
        (`self.DeLadoComFrenteADireita`)
        (else
          (`KismetSystemLibrary.PrintString` "Esquerda" true true (struct :`R` 1.0 :`B` 0.181547 :`A` 1.0) 10.0)
          (`self.DeLadoComFrenteAEsquerda`))))))

(event `DeLadoComFrenteAEsquerda`
  ;[1 1 1] Definir ponto de Saida
  (bind _output_get (set `self.BeginPosition` (`KismetMathLibrary.MakeVector` (.x (`SceneComponent.K2_GetComponentLocation` (`self.Cube`))) (- (.y (`SceneComponent.K2_GetComponentLocation` (`self.Cube`))) -100.0) (.z (`SceneComponent.K2_GetComponentLocation` (`self.Cube`))))))
  (`KismetSystemLibrary.DrawDebugBox` _output_get (10.0 10.0 10.0) (struct :`R` 1.0 :`G` 0.93951 :`A` 1.0) (struct) 1000.0)
  (`self.K2_SetActorLocation` (`self.AimPoint`) _output_get false true)
  (`self.Move`))

(event `self.ReceiveActorBeginOverlap`
  (params (OtherActor :type "Actor Object Reference"))
  (if (`self.ActorHasTag` OtherActor "Enemy")
    (bind _ascharacter (cast `Character` OtherActor))
    (set `self.EnemyInRange` _ascharacter)
    (`self.AttatchToArm`)))

(event `DeFrenteComFrenteADireita`
  ;[1 1 1] Definir ponto de Saida
  (bind _output_get (set `self.BeginPosition` (`KismetMathLibrary.MakeVector` (- (.x (`SceneComponent.K2_GetComponentLocation` (`self.Cube`))) 100.0) (.y (`SceneComponent.K2_GetComponentLocation` (`self.Cube`))) (.z (`SceneComponent.K2_GetComponentLocation` (`self.Cube`))))))
  (`KismetSystemLibrary.DrawDebugBox` _output_get (10.0 10.0 10.0) (struct :`R` 0.128808 :`G` 0.976124 :`B` 1.0 :`A` 1.0) (struct) 1000.0)
  (`self.K2_SetActorLocation` (`self.AimPoint`) _output_get false true)
  (`self.Move`))

(event `self.ReceiveActorEndOverlap`
  (params (OtherActor :type "Actor Object Reference"))
  (if (`self.ActorHasTag` "Enemy")
    (cast `Character` OtherActor)
    (set `self.EnemyInRange` null)))

(event `DeFrenteComFrenteAEsquerda`
  ;[1 1 1] Definir ponto de Saida
  (bind _output_get (set `self.BeginPosition` (`KismetMathLibrary.MakeVector` (- (.x (`SceneComponent.K2_GetComponentLocation` (`self.Cube`))) -100.0) (.y (`SceneComponent.K2_GetComponentLocation` (`self.Cube`))) (.z (`SceneComponent.K2_GetComponentLocation` (`self.Cube`))))))
  (`KismetSystemLibrary.DrawDebugBox` _output_get (10.0 10.0 10.0) (struct :`R` 1.0 :`G` 0.882571 :`A` 1.0) (struct) 1000.0)
  (`self.K2_SetActorLocation` (`self.AimPoint`) _output_get false true)
  (`self.Move`))

(event `self.ReceiveTick`
  (params (DeltaSeconds :type "Float (single-precision)")))

(event `Move`
  (bind _projectilemovement (`self.ProjectileMovement`))
  (bind _output (`|GetArrayItem` (`self.GetComponentsByTag` (`self.EnemyInRange`) "/Script/Engine.SceneComponent" "Pivot")))
  (`/Engine/EditorBlueprintResources/StandardMacros.IsValid` (`self.EnemyInRange`)
    (:`Is Valid`
      (`/Engine/EditorBlueprintResources/StandardMacros.IsValid` _output
        (:`Is Valid`
          ;[1 1 1] Set Enemy como target do braço
          (set `ProjectileMovementComponent.HomingTargetComponent` _output _projectilemovement)
          (set `ProjectileMovementComponent.bIsHomingProjectile` true _projectilemovement)
          (`KismetSystemLibrary.Delay` 1.0)
          (set `ProjectileMovementComponent.HomingTargetComponent` (`self.GetComponentByClass` (`self.AimPoint`) "/Script/Engine.SceneComponent") _projectilemovement)
          (`KismetSystemLibrary.Delay` 1.0)
          (set `ProjectileMovementComponent.bIsHomingProjectile` false _projectilemovement))))))

(event `AttatchToArm`
  (bind _enemyinrange (`self.EnemyInRange`))
  (`KismetSystemLibrary.PrintString` "Fuck" true true (struct :`R` 0.547339 :`G` 1.0 :`B` 0.294352 :`A` 1.0) 10.0)
  (`/Engine/EditorBlueprintResources/StandardMacros.IsValid` _enemyinrange
    (:`Is Valid`
      (`PrimitiveComponent.SetCollisionEnabled` (`Character.CapsuleComponent` _enemyinrange) "QueryOnly")
      (`PhysicsConstraintComponent.SetConstrainedComponents` (`self.PhysicsConstraint`) (`self.Cube`) "None" (`Character.Mesh` (`self.EnemyInRange`)) "Shoulder_Joint_L")
      (message `/Game/Interfaces/RaggdollKill.Kill Actor` (`self.EnemyInRange`))
      (`KismetSystemLibrary.Delay` 1.0)
      (`self.K2_DestroyActor` (`self.EnemyInRange`)))))

(fn `UserConstructionScript`)