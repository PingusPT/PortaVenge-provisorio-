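; Bp_AiCharacter is an AI guard character that walks a looping patrol between points in its PatrolLocation array.
; BeginPlay sets its Sphere component to ignore the Camera channel, resets the index and starts the patrol.
; GuardPatrol sets walk speed and runs AI MoveTo; on success it waits a short random delay, advances through three points with wraparound and calls itself again.
; A failed move has no handling.
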(event `self.ReceiveBeginPlay`
  (`PrimitiveComponent.SetCollisionResponseToChannel` (`self.Sphere`) "ECC_Camera" "ECR_Ignore")
  (set `self.Locations` 0)
  (`self.initialPatrol`))

(event `GuardPatrol`
  (set `CharacterMovementComponent.MaxWalkSpeed` 300.0 (`self.CharacterMovement`) :!label _label)
  (`|AIMoveTo` self (`|GetArrayItem` (`self.PatrolLocation`) (`self.Locations`)) null
    (:`OnSuccess`
      (`KismetSystemLibrary.Delay` (`KismetMathLibrary.RandomFloatInRange` 0.0 3.0))
      (`/Engine/EditorBlueprintResources/StandardMacros.IncrementInt` (`self.Locations`)
        (:`  `
          (if (> (`self.Locations`) 2)
            (set `self.Locations` 0))
          (`self.GuardPatrol`))))))

(event `initialPatrol`
  (goto _label))

(fn `UserConstructionScript`)