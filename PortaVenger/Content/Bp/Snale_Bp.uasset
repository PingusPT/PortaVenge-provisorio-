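; Snake actor for a minigame that detects losing on walls and winning at a finish.
; On each actor overlap it checks the other actor for static mesh components tagged WallSnake and for a FinalSnake actor tag.
; Either match teleports the snake to a fixed world location and calls SnakeLostGame or SnakeWinGame respectively.
; The Blueprint contains no movement logic, and a leftover debug string prints on every overlap.
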(event `self.ReceiveActorBeginOverlap`
  (params (OtherActor :type "Actor Object Reference"))
  ;[1 1 1] Colide With Something
  (`KismetSystemLibrary.PrintString` "AAAAAAAAAAAAAa")
  (`|ExecutionSequence`
    (:`then_0`
      (for _array_element (`self.GetComponentsByTag` OtherActor "/Script/Engine.StaticMeshComponent" "WallSnake")
        (if (`ActorComponent.ComponentHasTag` _array_element "WallSnake")
          (`self.K2_SetActorLocation` (0.0 1000.0 0.0))
          (`self.SnakeLostGame`))))
    (:`then_1`
      (if (`self.ActorHasTag` OtherActor "FinalSnake")
        (`self.K2_SetActorLocation` (0.0 1000.0 0.0))
        (`self.SnakeWinGame`)))))

(fn `UserConstructionScript`)