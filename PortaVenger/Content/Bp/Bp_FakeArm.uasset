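; Fake arm pawn that moves toward a nearby character's right shoulder to grab it.
; Overlap events track the character as EnemyInRange, and GrabEnemy sets a flag if one is valid.
; Tick then issues a single AIMoveTo to the OmbroDireito bone location through a DoOnce that never resets.
; Attach, physics and movement-disable nodes are unconnected, and the stored start position is unused.
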(event `self.ReceiveBeginPlay`
  (set `self.BeginPosition` (`self.K2_GetActorLocation`))
  (set `self.isMovingTo` false))

(event `self.ReceiveTick`
  (params (DeltaSeconds :type "Float (single-precision)"))
  (bind _mesh (`Character.Mesh` (`self.EnemyInRange`)))
  (if (`self.isMovingTo`)
    (`/Engine/EditorBlueprintResources/StandardMacros.DoOnce` false
      (:`Completed`
        (`|AIMoveTo` self (`SceneComponent.GetSocketLocation` _mesh (`SkinnedMeshComponent.GetSocketBoneName` _mesh "OmbroDireito")) null)))))

(event `self.ReceiveActorBeginOverlap`
  (params (OtherActor :type "Actor Object Reference"))
  (bind _ascharacter (cast `Character` OtherActor))
  (set `self.EnemyInRange` _ascharacter))

(event `self.ReceiveActorEndOverlap`
  (params (OtherActor :type "Actor Object Reference"))
  (cast `Character` OtherActor)
  (set `self.EnemyInRange` null))

(fn `GrabEnemy`
  (`/Engine/EditorBlueprintResources/StandardMacros.IsValid` (`self.EnemyInRange`)
    (:`Is Valid`
      (set `self.isMovingTo` true))))

(fn `UserConstructionScript`)