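; Gameplay controller that handles hotbar ability selection, character ability keys, the game-over screen with slow motion, and the CCTV-hacking snake minigame.
; BeginPlay spawns the snake and hotbar, caches camera and minigame references, and binds hack, win and lose events.
; The RTS camera's hack event toggles hacking, during which Tick moves the snake along the arrow-key direction.
; Win or loss resets the snake, broadcasts the result and updates the stored CCTV.
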(event `InputAction|SelectedAbility1`
  (params (Key :type "Key Structure"))
  (:`Pressed`
    (bind _output_get (set `self.SelectAbilityIndex` 0))
    (`/Game/Widgets/Hotbar/HotBar.UpdateSelectedAbility` (`self.HotBarReference`) _output_get)))

(event `InputAction|SelectedAbility2`
  (params (Key :type "Key Structure"))
  (:`Pressed`
    (bind _output_get (set `self.SelectAbilityIndex` 1))
    (`/Game/Widgets/Hotbar/HotBar.UpdateSelectedAbility` (`self.HotBarReference`) _output_get)))

(event `InputAction|SelectedAbility3`
  (params (Key :type "Key Structure"))
  (:`Pressed`
    (bind _output_get (set `self.SelectAbilityIndex` 2))
    (`/Game/Widgets/Hotbar/HotBar.UpdateSelectedAbility` (`self.HotBarReference`) _output_get)
    (`/Game/Bp/Bp_Character.Throw Coin` (`self.X1`))))

(event `InputAction|UpArrow`
  (params (Key :type "Key Structure"))
  ;[1 1 1] Snake Control Input
  (:`Pressed`
    (set `self.SnakeDir` (0.0 0.0 1.0))
    (if (`self.isHacking`) :!label _label
      (`FMODAudioComponent.Play` (`self.GetComponentByClass` (`self.Snake`) "/Script/FMODStudio.FMODAudioComponent")))))

(event `Key|J`
  (params (Key :type "Key Structure"))
  (:`Pressed`
    (bind _returnvalue (`|CreateWidget` "/Game/Widgets/GameOver/GameOver.GameOver_C" :!label _label_2))
    (`UserWidget.AddToViewport` _returnvalue 0)
    (`/Engine/EditorBlueprintResources/StandardMacros.DoOnce` false
      (:`Completed`
        (`GameplayStatics.SetGlobalTimeDilation` 0.5)
        (`/Game/Widgets/GameOver/GameOver.Fadeout` _returnvalue)
        (`Widget.RemoveFromParent` (`self.HotBarReference`))))))

(event `InputAction|DownArrow`
  (params (Key :type "Key Structure"))
  ;[1 1 1] Snake Control Input
  (:`Pressed`
    (set `self.SnakeDir` (0.0 0.0 -1.0))
    (goto _label)))

(event `DeathWidget`
  (goto _label_2))

(event `InputAction|LeftArrow`
  (params (Key :type "Key Structure"))
  ;[1 1 1] Snake Control Input
  (:`Pressed`
    (set `self.SnakeDir` (0.0 -1.0 0.0))
    (goto _label)))

(event `InputAction|RightArrow`
  (params (Key :type "Key Structure"))
  ;[1 1 1] Snake Control Input
  (:`Pressed`
    (set `self.SnakeDir` (0.0 1.0 -0.0))
    (goto _label)))

(event `self.ReceiveBeginPlay`
  (bind _returnvalue (`self.GetComponentByClass` (`self.SnakeMiniGame`) "/Script/Engine.ArrowComponent"))
  (bind _returnvalue_2 (`self.GetComponentByClass` (`self.SnakeMiniGame`) "/Script/Engine.CameraComponent"))
  (bind _returnvalue_3 (`self.GetComponentByClass` (`self.RtsCam`) "/Script/Engine.SpringArmComponent"))
  (bind _returnvalue_4 (`self.GetComponentByClass` (`self.RtsCam`) "/Script/Engine.CameraComponent"))
  (`|ExecutionSequence`
    (:`then_0`
      (bind _returnvalue_5 (`|SpawnActorFromClass` "/Game/Bp/Snale_Bp.Snale_Bp_C" (`KismetMathLibrary.MakeTransform` (0.0 1000.0 0.0)) "Undefined" "MultiplyWithRoot" null null))
      (bind _assnale_bp (cast `/Game/Bp/Snale_Bp` _returnvalue_5))
      (add `/Game/Bp/Snale_Bp.SnakeLostGame` _assnale_bp (delegate `LostSnakeGame`))
      (add `/Game/Bp/Snale_Bp.SnakeWinGame` _assnale_bp (delegate `SnakeWinGame_Event`))
      (set `self.Snake` _assnale_bp))
    (:`then_1`
      (bind _returnvalue_6 (`GameplayStatics.GetActorOfClass` "/Game/Bp/SnakeMiniGame.SnakeMiniGame_C"))
      (set `self.SnakeMiniGame` _returnvalue_6)
      (bind _asrts_camera (cast `/Game/Bp/Rts_Camera` (`GameplayStatics.GetPlayerPawn` 0))
        (:`then`
          (set `self.RtsCam` _asrts_camera))
        (:`CastFailed`
          _))
      (add `/Game/Bp/Rts_Camera.HackingMode123` _asrts_camera (delegate `CameraHack`)))
    (:`then_2`
      (`/Engine/EditorBlueprintResources/StandardMacros.IsValid` _returnvalue
        (:`Is Valid`
          (set `self.ArrowPoint` _returnvalue))))
    (:`then_3`
      (`/Engine/EditorBlueprintResources/StandardMacros.IsValid` _returnvalue_4
        (:`Is Valid`
          (set `self.PlayerCam` _returnvalue_4))))
    (:`then_4`
      (`/Engine/EditorBlueprintResources/StandardMacros.IsValid` _returnvalue_3
        (:`Is Valid`
          (set `self.RtsSpring` _returnvalue_3))))
    (:`then_5`
      (set `self.isHacking` false)
      (`/Engine/EditorBlueprintResources/StandardMacros.IsValid` _returnvalue_2
        (:`Is Valid`
          (bind _output_get (set `self.MiniGameCamera` _returnvalue_2))
          (`ActorComponent.SetActive` _output_get false false))))
    (:`then_6`
      (set `self.Fmod Snake` (`self.GetComponentByClass` (`self.Snake`) "/Script/FMODStudio.FMODAudioComponent")))
    (:`then_7`
      (bind _returnvalue_7 (`|CreateWidget` "/Game/Widgets/Hotbar/HotBar.HotBar_C"))
      (bind _output_get_2 (set `self.HotBarReference` _returnvalue_7))
      (`UserWidget.AddToViewport` _output_get_2 0))
    (:`then_8`
      (bind _returnvalue_8 (`GameplayStatics.GetActorOfClass` "/Game/Bp/Bp_Character.Bp_Character_C"))
      (set `self.X1` _returnvalue_8))))

(event `Key|F`
  (params (Key :type "Key Structure"))
  (:`Pressed`
    (`/Game/Bp/Bp_Character.KnifeKill` (`self.X1`))))

(event `CameraHack`
  (bind _ishacking (`self.isHacking`))
  (bind _returnvalue_location (`KismetMathLibrary.BreakTransform` (`SceneComponent.K2_GetComponentToWorld` (`|GetArrayItem` (`self.GetComponentsByTag` (`self.SnakeMiniGame`) "/Script/Engine.SceneComponent" "Spawn")))))
  ;[1 1 1] Camera Go to Snake Game
  (set `self.isHacking` (not _ishacking))
  (if _ishacking
    (bind _assnale_bp (cast `/Game/Bp/Snale_Bp` (`self.Snake`)))
    (`/Game/Bp/Snale_Bp.Activate Trail` _assnale_bp)
    (`KismetSystemLibrary.PrintText` (`KismetTextLibrary.Conv_VectorToText` _returnvalue_location) true true (struct :`G` 0.66 :`B` 1.0 :`A` 1.0) 100000.0)
    (bind _output_get (set `self.SnakeLocation` _returnvalue_location))
    (`self.K2_SetActorLocation` (`self.Snake`) _output_get false false)))

(event `LostSnakeGame`
  ;[1 1 1] Lose Snake Game
  (set `self.isHacking` false)
  (set `self.SnakeDir` (0.0 0.0 0.0))
  (set `self.HackingSuccess` false)
  (`KismetSystemLibrary.Delay` 0.2 :!label _label_3)
  (`self.TurnOffCamera` (`self.HackingSuccess`))
  (`self.K2_SetActorLocation` (`self.Snake`) (`self.SnakeLocation`) false false)
  (`Widget.RemoveFromParent` (`self.Snake Widget`))
  (bind _asbp_cctv (cast `/Game/Bp/Bp_CCTV` (`self.Camera_0`)))
  (`/Game/Bp/Bp_CCTV.ResetWidget` _asbp_cctv))

(event `self.ReceiveTick`
  (params (DeltaSeconds :type "Float (single-precision)"))
  ;[1 1 1] Add Movement to Snake
  (if (`self.isHacking`)
    (`self.K2_AddActorLocalOffset` (`self.Snake`) (* (`self.SnakeDir`) DeltaSeconds 500.0) true false)))

(event `SnakeWinGame_Event`
  ;[1 1 1] Win Snake Game
  (set `self.isHacking` false)
  (set `self.SnakeDir` (0.0 0.0 0.0))
  (set `self.HackingSuccess` true)
  (bind _asbp_cctv (cast `/Game/Bp/Bp_CCTV` (`self.Camera_0`)))
  (`/Game/Bp/Bp_CCTV.EnableSpawks` _asbp_cctv)
  (`/Game/Bp/Bp_CCTV.Camera_Off` _asbp_cctv)
  (goto _label_3))

(event `/Game/Interfaces/SparklCam.Sparkle`
  (params (Camera :type "Actor Object Reference") (SnakeWidget :type "/Game/Widgets/Snake/Snake_Minigame_Widget Object Reference"))
  (set `self.Camera_0` Camera)
  (set `self.Snake Widget` SnakeWidget))

(fn `UserConstructionScript`)