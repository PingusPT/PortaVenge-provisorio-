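; Test trigger volume that scales the player character's footstep reverb by proximity to the area's origin.
; Overlap events track actors tagged Player, and the first in-range Tick stores their squared distance as the maximum, never reset afterwards.
; While in range, Tick sends one minus the squared-distance ratio to Bp_Character's UpdateReverbFootStep.
; It also prints that value and draws a long-lived debug box on BeginPlay.
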(event `self.ReceiveBeginPlay`
  (bind (_origin _boxextent) (`KismetSystemLibrary.GetComponentBounds` (`self.Box`)))
  (set `self.ActorInRange` false)
  (`KismetSystemLibrary.DrawDebugBox` _origin _boxextent (struct :`R` 1.0 :`B` 0.042296 :`A` 1.0) (struct) 100000.0 10.0))

(event `self.ReceiveActorBeginOverlap`
  (params (OtherActor :type "Actor Object Reference"))
  (if (`self.ActorHasTag` OtherActor "Player")
    (set `self.Other Actor` OtherActor)
    (set `self.ActorInRange` true)))

(event `self.ReceiveActorEndOverlap`
  (params (OtherActor :type "Actor Object Reference"))
  (if (`self.ActorHasTag` OtherActor "Player")
    (set `self.ActorInRange` false)))

(event `self.ReceiveTick`
  (params (DeltaSeconds :type "Float (single-precision)"))
  (bind _returnvalue (`KismetMathLibrary.FClamp` (/ (`KismetMathLibrary.Vector_DistanceSquared` (`self.K2_GetActorLocation` (`self.Other Actor`)) (`self.K2_GetActorLocation`)) 1000.0) 0.0 10000.0))
  (bind _returnvalue_2 (- 1.0 (/ _returnvalue (`self.Set MaxDistance`))))
  (if (`self.ActorInRange`)
    (`|ExecutionSequence`
      (:`then_0`
        (`/Engine/EditorBlueprintResources/StandardMacros.DoOnce` false
          (:`Completed`
            (set `self.Set MaxDistance` _returnvalue))))
      (:`then_1`
        (`KismetSystemLibrary.PrintString` (`KismetStringLibrary.Conv_DoubleToString` _returnvalue_2))
        (bind _asbp_character (cast `/Game/Bp/Bp_Character` (`self.Other Actor`)))
        (`/Game/Bp/Bp_Character.UpdateReverbFootStep` _asbp_character _returnvalue_2)))))

(fn `UserConstructionScript`)