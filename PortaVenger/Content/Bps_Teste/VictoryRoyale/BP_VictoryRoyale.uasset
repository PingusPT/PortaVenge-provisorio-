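; BP_VictoryRoyale is a victory trigger that ends the level once all enemies are gone.
; When a Bp_Character overlaps its Box, it reads EnemyInGame from Main_GameMode and proceeds only if the count is zero or less.
; A DoOnce then shows the Level1to2 widget and plays WinGame, so the win fires a single time.
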(event `self.Box.OnComponentBeginOverlap`
  (params (OverlappedComponent :type "PrimitiveComponent Object Reference") (OtherActor :type "Actor Object Reference") (OtherComp :type "PrimitiveComponent Object Reference") (OtherBodyIndex :type Integer) (bFromSweep :type Boolean) (SweepResult :type "HitResult Structure (by ref)"))
  (cast `/Game/Bp/Bp_Character` OtherActor)
  (bind _asmain_game_mode (cast `/Game/Bp/Main_GameMode` (`GameplayStatics.GetGameMode`)))
  (if (<= (`/Game/Bp/Main_GameMode.EnemyInGame` _asmain_game_mode) 0)
    (`/Engine/EditorBlueprintResources/StandardMacros.DoOnce` false
      (:`Completed`
        (bind _returnvalue (`|CreateWidget` "/Game/Widgets/WidgetLevelPassed/Level1to2.Level1to2_C"))
        (`UserWidget.AddToViewport` _returnvalue 0)
        (`FMODAudioComponent.Play` (`self.WinGame`))))))

(fn `UserConstructionScript`)