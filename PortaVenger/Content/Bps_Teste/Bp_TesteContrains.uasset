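; Test actor for physics constraints that hooks an overlapping Bp_Character onto a physics-simulated Sphere.
; One second after BeginPlay, its PhysicsConstraint links Sphere to Cube and Sphere starts simulating physics.
; On overlap with the character, it prints a debug message, teleports that same constraint to the character, enables mesh physics and re-targets the constraint to link mesh and Sphere.
; Actor-attach and Timeline nodes are left unconnected.
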(event `self.ReceiveBeginPlay`
  (`KismetSystemLibrary.Delay` 1.0)
  (`PhysicsConstraintComponent.SetConstrainedComponents` (`self.PhysicsConstraint`) (`self.Sphere`) "None" (`self.Cube`) "None")
  (`PrimitiveComponent.SetSimulatePhysics` (`self.Sphere`) true))

(event `self.ReceiveActorBeginOverlap`
  (params (OtherActor :type "Actor Object Reference"))
  (bind _asbp_character (cast `/Game/Bp/Bp_Character` OtherActor))
  (`KismetSystemLibrary.PrintString` "YAOOO" true true (struct :`R` 1.0 :`G` 0.120715 :`A` 1.0))
  (`SceneComponent.K2_SetWorldLocation` (`self.PhysicsConstraint`) (`self.K2_GetActorLocation` _asbp_character) false true)
  (bind _mesh (`Character.Mesh` _asbp_character))
  (`PrimitiveComponent.SetSimulatePhysics` _mesh true)
  (`PhysicsConstraintComponent.SetConstrainedComponents` (`self.PhysicsConstraint`) _mesh "None" (`self.Sphere`) "None"))

(fn `UserConstructionScript`)