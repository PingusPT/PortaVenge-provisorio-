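; BP_LuzTEste is a rotating light actor with two spotlights and FMOD audio, all off at BeginPlay.
; Activate turns on both lights once, playing the sound at low volume unless IsCutscene is set.
; It also runs the Spin timeline to drive root world pitch, calling itself on finish to loop endlessly.
; Desligarsom stops only the audio.
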(event `self.ReceiveBeginPlay`
  (`LightComponent.SetIntensity` (`self.SpotLight2`) 0.0)
  (`LightComponent.SetIntensity` (`self.SpotLight1`) 0.0)
  (`FMODAudioComponent.Stop` (`self.FMODAudio`)))

(event `Activate`
  (bind _defaultsceneroot (`self.DefaultSceneRoot`))
  (bind _fmodaudio (`self.FMODAudio`))
  (bind (_returnvalue_roll _returnvalue_pitch _returnvalue_yaw) (`KismetMathLibrary.BreakRotator` (`SceneComponent.K2_GetComponentRotation` _defaultsceneroot)))
  (`|ExecutionSequence`
    (:`then_0`
      (`/Engine/EditorBlueprintResources/StandardMacros.DoOnce` false
        (:`Completed`
          (`LightComponent.SetIntensity` (`self.SpotLight2`) 1000.0)
          (`LightComponent.SetIntensity` (`self.SpotLight1`) 1000.0)
          (if (not (`self.IsCutscene`))
            (`FMODAudioComponent.Play` _fmodaudio)
            (`FMODAudioComponent.SetVolume` _fmodaudio 0.2)))))
    (:`then_1`
      (bind (_direction _newtrack_0) (`Timeline|Spin` :!via `PlayFromStart`)
        (:`Update`
          (`SceneComponent.K2_SetWorldRotation` _defaultsceneroot (`KismetMathLibrary.MakeRotator` _returnvalue_roll _newtrack_0 _returnvalue_yaw) false false))
        (:`Finished`
          (`self.Activate`))))))

(event `Desligar som`
  (`FMODAudioComponent.Stop` (`self.FMODAudio`)))

(fn `UserConstructionScript`)