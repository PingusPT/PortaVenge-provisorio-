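; Dialogue trigger actor that starts a dialogue when the player's body enters its box.
; On overlap with a component tagged PlayerBody, it creates a DialoguesBP widget, adds it to the viewport and passes its dialogue lines and speaker.
; It then disables RTS camera movement through Main_GameMode, hands that camera to the widget and destroys itself, making the trigger one-shot.
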(event `self.Box.OnComponentBeginOverlap`
  (params (OverlappedComponent :type "PrimitiveComponent Object Reference") (OtherActor :type "Actor Object Reference") (OtherComp :type "PrimitiveComponent Object Reference") (OtherBodyIndex :type Integer) (bFromSweep :type Boolean) (SweepResult :type "HitResult Structure (by ref)"))
  (if (`ActorComponent.ComponentHasTag` OtherComp "PlayerBody")
    (bind _returnvalue (`|CreateWidget` "/Game/Dialogues/DialoguesBP.DialoguesBP_C"))
    (`UserWidget.AddToViewport` _returnvalue 0)
    (set `/Game/Dialogues/DialoguesBP.TestArray` (`self.Dialogos`) _returnvalue)
    (set `/Game/Dialogues/DialoguesBP.WhoIsYapping` (`self.WhoIsYapping`) _returnvalue)
    (bind _asmain_game_mode (cast `/Game/Bp/Main_GameMode` (`GameplayStatics.GetGameMode`)))
    (bind _as_rts_camera (`/Game/Bp/Main_GameMode.As Rts Camera` _asmain_game_mode))
    (set `/Game/Bp/Rts_Camera.isMovementX1Disabled` true _as_rts_camera)
    (`/Game/Dialogues/DialoguesBP.Get RtsCam` _returnvalue _as_rts_camera)
    (`self.K2_DestroyActor`)))

(fn `UserConstructionScript`)