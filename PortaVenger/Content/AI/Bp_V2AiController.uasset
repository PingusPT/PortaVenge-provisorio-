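; AI controller for stealth enemies that runs BT_NewEnemy and feeds it state, senses and locations through the Blackboard.
; Player sightings animate two line-of-sight components, after a random delay at longer range.
; Dead bodies and tagged noises (coin, portal, player) set sense states and play throttled FMOD reactions, with noises expiring by timer.
; It also toggles vision and outline display on click, and sphere-traces to shift patrol points around other enemies.
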(event `/Game/Interfaces/SetEnemySate.SetEnemyState`
  (params (State :type "/Game/AI/EQS/EnemyState Enum" :default "NewEnumerator0"))
  (bind _output_get (set `self.EnemyState` State))
  (`BlackboardComponent.SetValueAsEnum` (`self.Blackboard`) "State" _output_get)
  (`KismetSystemLibrary.PrintString` (`|GetEnumeratorNameAsString` _output_get)))

(event `Set Sense State`
  (params (SenseState :type "/Game/AI/EQS/SenseState Enum" :default "NewEnumerator0"))
  (bind _output_get (set `self.SenseState` SenseState))
  (`BlackboardComponent.SetValueAsEnum` (`self.Blackboard`) "SenseState" _output_get)
  (`KismetSystemLibrary.PrintString` (`|GetEnumeratorNameAsString` _output_get)))

(event `ClickEvent`
  (bind _zonadevisao (`self.ZonaDeVisao`))
  (bind _mesh (`Character.Mesh` (`self.ControlledPawn`)))
  (`|ExecutionSequence`
    (:`then_0`
      (if (`self.OutlineEnabled`)
        (`SceneComponent.SetHiddenInGame` _zonadevisao (not (`SceneComponent.bHiddenInGame` _zonadevisao)) false)
        (`SceneComponent.SetHiddenInGame` (`self.ZonaDeVisao1`) (not (`SceneComponent.bHiddenInGame` _zonadevisao)) false)
        (else
          (if (`self.ClickOutline`) :!label _label
            (set `self.ClickOutline` false)
            (`PrimitiveComponent.SetRenderCustomDepth` _mesh true)
            (`SceneComponent.SetHiddenInGame` (`self.ZonaDeVisao1`) false false)
            (`SceneComponent.SetHiddenInGame` (`self.ZonaDeVisao`) false false)
            (else
              (set `self.ClickOutline` true)
              (`PrimitiveComponent.SetRenderCustomDepth` _mesh false)
              (`SceneComponent.SetHiddenInGame` (`self.ZonaDeVisao1`) true false)
              (`SceneComponent.SetHiddenInGame` (`self.ZonaDeVisao`) true false))))))
    (:`then_1`
      (`/Engine/EditorBlueprintResources/StandardMacros.DoOnce` false
        (:`Completed`
          (goto _label))))))

(event `self.ReceiveBeginPlay`
  (bind _output (`|GetArrayItem` (`self.GetComponentsByTag` (`self.K2_GetPawn`) "/Script/LineOfSight.LineOfSightComponent" "ZonaDeVisao")))
  (`self.RunBehaviorTree` "/Game/AI/BT_NewEnemy.BT_NewEnemy")
  (set `self.ActorDead` false)
  (`KismetSystemLibrary.Delay` 0.4)
  (`/Engine/EditorBlueprintResources/StandardMacros.IsValid` _output
    (:`Is Valid`
      (set `self.ZonaDeVisao` _output)
      (set `self.ZonaDeVisao1` (`|GetArrayItem` (`self.GetComponentsByTag` (`self.K2_GetPawn`) "/Script/LineOfSight.LineOfSightComponent" "ZonaDeVisao1")))
      (set `self.Ns_Questao` (`self.GetComponentByClass` (`self.K2_GetPawn`) "/Script/Niagara.NiagaraComponent"))
      (bind _ascharacter (cast `Character` (`self.K2_GetPawn`)))
      (bind _output_get (set `self.ControlledPawn` _ascharacter))
      (set `self.Fmod Audio` (`self.GetComponentByClass` _output_get "/Script/FMODStudio.FMODAudioComponent"))
      (bind _output_get_2 (set `self.InitialRotation` (`self.K2_GetActorRotation` (`self.ControlledPawn`))))
      (`BlackboardComponent.SetValueAsRotator` (`self.Blackboard`) "LookAt" _output_get_2)
      (`KismetSystemLibrary.K2_SetTimerDelegate` (delegate `Check navigation`) 0.2 true)
      (cast `/Game/AI/Bp_AiEnemy` (`self.ControlledPawn`)
        (:`then`
          (`FMODAudioComponent.SetEvent` (`self.DesconfiadoMorto`) "/Game/FMOD/Events/INIMIGOS/InimigoPequeno/DesconfiaMORTO_IP.DesconfiaMORTO_IP")
          (`FMODAudioComponent.SetEvent` (`self.DesconfiadoSom`) "/Game/FMOD/Events/INIMIGOS/InimigoPequeno/DesconfiaSOM_IP.DesconfiaSOM_IP"))
        (:`CastFailed`
          (`FMODAudioComponent.SetEvent` (`self.DesconfiadoMorto`) "/Game/FMOD/Events/INIMIGOS/InimigoGordo/DesconfiaMORTO_IG.DesconfiaMORTO_IG")
          (`FMODAudioComponent.SetEvent` (`self.DesconfiadoSom`) "/Game/FMOD/Events/INIMIGOS/InimigoPequeno/DesconfiaSOM_IP.DesconfiaSOM_IP"))))
    (:`Is Not Valid`
      (`KismetSystemLibrary.PrintString` (`KismetSystemLibrary.GetDisplayName` self)))))

(event `Check navigation`
  (bind _returnvalue (`self.K2_GetActorLocation` (`self.ControlledPawn`)))
  (bind _outhit (`KismetSystemLibrary.SphereTraceSingle` _returnvalue (+ _returnvalue (* (`self.GetActorForwardVector` (`self.ControlledPawn`)) 250.0)) 70.0 "TraceTypeQuery11" false (`|MakeArray` (`self.ControlledPawn`) :!type "Actor Object Reference") "ForDuration" true (struct :`R` 1.0 :`A` 1.0) (struct :`G` 1.0 :`A` 1.0) 0.5))
  (bind (_bblockinghit _binitialoverlap _time _distance _location _impactpoint _normal _impactnormal _physmat _hitactor) (`GameplayStatics.BreakHitResult` _outhit))
  (if _bblockinghit
    (if (`self.ActorHasTag` _hitactor "Enemy")
      (bind _asbp_ai_enemy (cast `/Game/AI/Bp_AiEnemy` (`self.ControlledPawn`)))
      (bind _output_get (set `/Game/AI/Bp_AiEnemy.CurrentPatrolPoint` (`KismetMathLibrary.MakeVector` (.x (+ (`self.K2_GetActorLocation` (`self.ControlledPawn`)) (* (`self.GetActorForwardVector` (`self.ControlledPawn`)) 300.0) (* (`self.GetActorRightVector` (`self.ControlledPawn`)) 300.0))) (.y (+ (`self.K2_GetActorLocation` (`self.ControlledPawn`)) (* (`self.GetActorForwardVector` (`self.ControlledPawn`)) 300.0) (* (`self.GetActorRightVector` (`self.ControlledPawn`)) 300.0)))) _asbp_ai_enemy))
      (`BlackboardComponent.SetValueAsVector` (`self.Blackboard`) "PatrolLocations" _output_get)
      (`KismetSystemLibrary.DrawDebugBox` _output_get (10.0 10.0 10.0) (struct :`R` 1.0 :`G` 0.039648 :`A` 1.0) (struct) 10000.0 10.0))))

(event `self.ReceiveTick`
  (params (DeltaSeconds :type "Float (single-precision)"))
  (if (not (`self.ActorDead`))
    (switch `/Game/AI/EQS/EnemyState` "NewEnumerator0"
      (:`NewEnumerator0`
        (`BlackboardComponent.SetValueAsRotator` (`self.Blackboard`) "LookAt" (`self.InitialRotation`))))))

(event `Recive Vision Of Player`
  (params (NewParam :type "/Game/Bp/Bp_Character Object Reference") (`Player location` :type "Vector Structure"))
  (bind _zonadevisao (`self.ZonaDeVisao`))
  (`LineOfSightComponent.StopInterpRadius` (`self.ZonaDeVisao1`))
  (`LineOfSightComponent.StopInterpRadius` (`self.ZonaDeVisao`))
  (`LineOfSightComponent.StopInterpAngle` (`self.ZonaDeVisao`))
  ;[0 0 0] Viu o Player
  (`BlackboardComponent.SetValueAsObject` (`self.Blackboard`) "Player" NewParam)
  (`BlackboardComponent.SetValueAsBool` (`self.Blackboard`) "asSeenPlayer?" true)
  (bind _output_get (set `self.PlayerSeenLocation` `Player location`))
  (`/Game/Interfaces/SetEnemySate.SetEnemyState` "NewEnumerator2")
  (if (< (`KismetMathLibrary.Vector_Distance` _output_get (`self.K2_GetActorLocation` (`self.K2_GetPawn`))) 750.0)
    (`|ExecutionSequence` :!label _label_2
      (:`then_0`
        (`LineOfSightComponent.StartInterpRadius` _zonadevisao 50.0 (`self.RadiusLineOfSight2`) 400.0 0.0)
        (`LineOfSightComponent.StartInterpAngle` _zonadevisao 30.0 30.0 400.0 0.0)
        (`KismetSystemLibrary.Delay` 2.0)
        (`ActorComponent.Deactivate` (`self.Ns_Questao`)))
      (:`then_1`
        (`LineOfSightComponent.StartInterpRadius` (`self.ZonaDeVisao1`) 50.0 (`self.RadiusLineOfSight2`) 0.0 400.0)))
    (else
      (set `self.randomTime` (`KismetMathLibrary.RandomFloatInRange` 0.5 1.0))
      (bind _returnvalue (`KismetSystemLibrary.K2_SetTimerDelegate` (delegate `Detect Playe`) (`self.randomTime`)))
      (set `self.Timer` _returnvalue)
      (`ActorComponent.Activate` (`self.Ns_Questao`) false))))

(event `Detect Playe`
  ;[0 0 0] Viu o Player
  (`KismetSystemLibrary.PrintString` "Fez o Timer" true true (struct :`R` 1.0 :`G` 0.10015 :`A` 1.0))
  (goto _label_2))

(event `Recive EndOverlap`
  (bind _zonadevisao (`self.ZonaDeVisao`))
  (`KismetSystemLibrary.K2_ClearAndInvalidateTimerHandle` (`self.Timer`))
  (`LineOfSightComponent.StopInterpRadius` (`self.ZonaDeVisao1`))
  (`LineOfSightComponent.StopInterpRadius` (`self.ZonaDeVisao`))
  ;[0 0 0] Parou de ver o PLayer
  (`LineOfSightComponent.StopInterpAngle` (`self.ZonaDeVisao`))
  (`BlackboardComponent.SetValueAsBool` (`self.Blackboard`) "asSeenPlayer?" false)
  (`BlackboardComponent.SetValueAsVector` (`self.Blackboard`) "SeenLocation" (`self.PlayerSeenLocation`))
  (`|ExecutionSequence`
    (:`then_0`
      (`LineOfSightComponent.StartInterpRadius` _zonadevisao 50.0 (`self.RadiusLineOfSight2`) 400.0 400.0)
      (`LineOfSightComponent.StartInterpAngle` _zonadevisao 30.0 30.0 400.0 0.0))
    (:`then_1`
      (`LineOfSightComponent.StartInterpRadius` (`self.ZonaDeVisao1`) 50.0 50.0 0.0 400.0))))

(event `Viu Inimigo Morto`
  (params (`Viewed Actor` :type "Actor Object Reference"))
  (bind _asbp_ai_enemy (cast `/Game/AI/Bp_AiEnemy` `Viewed Actor`)
    (:`then`
      (bind _output_get (set `self.Viewed Actor` _asbp_ai_enemy))
      (`self.Set Sense State` "NewEnumerator2")
      (`BlackboardComponent.SetValueAsVector` (`self.Blackboard`) "SeenActorDead" (- (`self.K2_GetActorLocation` _output_get) (0.0 0.0 100.0)))
      (`/Game/Interfaces/SetEnemySate.SetEnemyState` "NewEnumerator1"))
    (:`CastFailed`
      (bind _asbp_ai_enemy_gordo (cast `/Game/AI/Bp_AiEnemyGordo` `Viewed Actor`))
      (set `self.Viewed Actor` _asbp_ai_enemy_gordo)
      (`self.Set Sense State` "NewEnumerator2")
      (`BlackboardComponent.SetValueAsVector` (`self.Blackboard`) "SeenActorDead" (`NavigationSystemV1.K2_GetRandomReachablePointInRadius` (`SceneComponent.K2_GetComponentLocation` (`|GetArrayItem` (`self.GetComponentsByTag` _asbp_ai_enemy_gordo "/Script/Engine.SceneComponent" "HelpPoint"))) 10.0 null null))))
  (`|ExecutionSequence`
    (:`then_0`
      (`/Engine/EditorBlueprintResources/StandardMacros.DoOnce` false :!label _label_3
        (:`Completed`
          (`FMODAudioComponent.Play` (`self.DesconfiadoMorto`)))))
    (:`then_1`
      (`KismetSystemLibrary.Delay` 6.0)
      (goto _label_3 :!via `Reset`))))

(event `Actor Go To Locatio`
  (params (Location :type "Vector Structure"))
  (`/Engine/EditorBlueprintResources/StandardMacros.DoOnce` false
    (:`Completed`
      (`KismetSystemLibrary.DrawDebugBox` Location (30.0 30.0 30.0) (struct :`R` 1.0 :`G` 0.095891 :`A` 1.0) (struct) 30.0 30.0)
      (`|AIMoveTo` (`self.K2_GetPawn`) Location null 10.0
        (:`OnSuccess`
          (`KismetSystemLibrary.PrintString` "Sucesso" true true (struct :`G` 1.0 :`B` 0.213701 :`A` 1.0)))
        (:`OnFail`
          (`KismetSystemLibrary.PrintString` "Falhou" true true (struct :`R` 1.0 :`B` 0.104549 :`A` 1.0)))))))

(event `DestroiVisiom`
  ;[0 0 0] Destroi Line of Sight
  (`ActorComponent.K2_DestroyComponent` (`self.ZonaDeVisao`))
  (`ActorComponent.K2_DestroyComponent` (`self.ZonaDeVisao1`))
  (`CharacterMovementComponent.DisableMovement` (`Character.CharacterMovement` (`self.ControlledPawn`))))

(event `Ouviu Algo`
  (params (`Audio Location` :type "Vector Structure") (Tag :type Name))
  (bind _audio_location (`self.Audio Location`))
  (set `self.Audio Location` `Audio Location`)
  (`BlackboardComponent.SetValueAsFloat` (`self.Blackboard`) "TimeSoundDelay" (`KismetMathLibrary.RandomFloatInRange` 5.6 6.0))
  (if (== Tag "Coin")
    (`self.Set Sense State` "NewEnumerator1")
    (`BlackboardComponent.SetValueAsVector` (`self.Blackboard`) "SoundLocation" (`self.Audio Location`))
    (`self.Set Audio VAr`)
    (`|ExecutionSequence` :!label _label_4
      (:`then_0`
        (`/Engine/EditorBlueprintResources/StandardMacros.DoOnce` false :!label _label_5
          (:`Completed`
            (`FMODAudioComponent.Play` (`self.DesconfiadoSom`)))))
      (:`then_1`
        (`KismetSystemLibrary.Delay` 3.0)
        (goto _label_5 :!via `Reset`)))
    (elif (== Tag "Portal")
      (`self.Set Sense State` "NewEnumerator0")
      (`BlackboardComponent.SetValueAsVector` (`self.Blackboard`) "SoundLocation" _audio_location)
      (`self.Set Audio VAr`)
      (`|ExecutionSequence`
        (:`then_0`
          (`/Engine/EditorBlueprintResources/StandardMacros.DoOnce` false :!label _label_6
            (:`Completed`
              (`FMODAudioComponent.Play` (`self.DesconfiadoPortal`)))))
        (:`then_1`
          (`KismetSystemLibrary.Delay` 5.0)
          (goto _label_6 :!via `Reset`)))
      (elif (== Tag "Player")
        (`self.Set Sense State` "NewEnumerator3")
        (`BlackboardComponent.SetValueAsVector` (`self.Blackboard`) "SoundLocation" _audio_location)
        (`KismetSystemLibrary.PrintString` "OUVIU PLAYER" true true (struct :`R` 1.0 :`B` 0.09376 :`A` 1.0))
        (`self.Set Audio VAr`)
        (goto _label_4)))))

(event `PlaySound Death`
  (`FMODAudioComponent.Play` (`self.Fmod Audio`)))

(event `Set Audio VAr`
  (set `self.EscotouAlgo` true)
  (bind _returnvalue (`KismetSystemLibrary.K2_SetTimerDelegate` (delegate `TurnOffSound`) (`BlackboardComponent.GetValueAsFloat` (`self.Blackboard`) "TimeSoundDelay")))
  (set `self.AudioTImer` _returnvalue)
  (`BlackboardComponent.SetValueAsBool` (`self.Blackboard`) "AsHearingSomething" true)
  (`/Game/Interfaces/SetEnemySate.SetEnemyState` "NewEnumerator1")
  (`KismetSystemLibrary.DrawDebugBox` (`BlackboardComponent.GetValueAsVector` (`self.Blackboard`) "SoundLocation") (10.0 10.0 10.0) (struct :`R` 1.0 :`G` 0.089367 :`B` 0.945098 :`A` 1.0) (struct) 100.0 10.0))

(event `TurnOffSound`
  (bind _output_get (set `self.EscotouAlgo` false))
  (`BlackboardComponent.SetValueAsBool` (`self.Blackboard`) "AsHearingSomething" _output_get))

(fn `UserConstructionScript`)