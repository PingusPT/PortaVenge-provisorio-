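; Enemy AI character that patrols along a spline and detects the player with a line-of-sight vision cone.
; Tick advances it along the spline, looping at the end, while ZonaDeVisao builds a hidden, toggleable mesh from line traces.
; Sighting a Player-tagged actor sets a blackboard flag and opens the death widget via the camera controller.
; Custom events handle removing vision, death sound and ragdoll death.
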(event `self.ReceiveTick`
  (params (DeltaSeconds :type "Float (single-precision)"))
  (bind _returnvalue (`SplineComponent.GetTransformAtDistanceAlongSpline` (`/Game/AI/Bp_Spline.Spline` (`self.Spline`)) (`self.DistanceAlongSpline`) "World" false))
  (`|ExecutionSequence`
    (:`then_0`
      (`/Engine/EditorBlueprintResources/StandardMacros.IsValid` (`self.Spline`)
        (:`Is Valid`
          (`|ExecutionSequence`
            (:`then_0`
              (if (`self.Patroling?`)
                (set `self.DistanceAlongSpline` (+ (* DeltaSeconds (`self.SplineSpeed`)) (`self.DistanceAlongSpline`)))
                (`SceneComponent.K2_SetRelativeTransform` (`self.CapsuleComponent`) (`KismetMathLibrary.MakeTransform` (`KismetMathLibrary.MakeVector` (.x (.location _returnvalue)) (.y (.location _returnvalue)) (+ (.z (.location _returnvalue)) -90.0)) (`KismetMathLibrary.MakeRotator` (.roll (.rotation _returnvalue)) (.pitch (.rotation _returnvalue)) (+ (.yaw (.rotation _returnvalue)) 0.0))) false false)
                (if (> (`self.DistanceAlongSpline`) (`SplineComponent.GetSplineLength` (`/Game/AI/Bp_Spline.Spline` (`self.Spline`))))
                  (set `self.DistanceAlongSpline` 0.0))))))))))

(event `Set Active FieldView`
  (bind _zonadevisao (`self.ZonaDeVisao`))
  (`SceneComponent.SetHiddenInGame` _zonadevisao (not (`SceneComponent.bHiddenInGame` _zonadevisao)) false))

(event `DestroiVisiom`
  (`ActorComponent.K2_DestroyComponent` (`self.ZonaDeVisao`))
  (set `self.Patroling?` false)
  (`CharacterMovementComponent.DisableMovement` (`self.CharacterMovement`)))

(event `PlaySound Death`
  (`FMODAudioComponent.Play` (`self.FMODAudio`)))

(event `/Game/Interfaces/RaggdollKill.Kill Actor`
  (if (not (`self.ActorDead?`))
    (`CharacterMovementComponent.DisableMovement` (`self.CharacterMovement`))
    (`ActorComponent.K2_DestroyComponent` (`self.FMODAudio`))
    (`PrimitiveComponent.SetSimulatePhysics` (`self.Weapon`) true)
    (`PrimitiveComponent.SetSimulatePhysics` (`self.Mesh`) true)
    (set `self.ActorDead?` true)
    (`PrimitiveComponent.SetCollisionResponseToChannel` (`self.Mesh`) "ECC_GameTraceChannel2" "ECR_Ignore")))

(event `self.ReceiveBeginPlay`
  (bind _zonadevisao (`self.ZonaDeVisao`))
  ;[1 1 1] New Line of Sight
  (`LineOfSightComponent.StartLineTrace` (`self.ZonaDeVisao`) "TraceTypeQuery1" 120)
  (`LineOfSightComponent.StartBuildMesh` (`self.ZonaDeVisao`))
  (set `self.ActorDead?` false)
  (add `LineOfSightComponent.BeginOverlap` _zonadevisao (delegate `FakeBegin Overlap`))
  (`SceneComponent.SetHiddenInGame` _zonadevisao true false))

(event `FakeBegin Overlap`
  (params (Hit :type "HitResult Structure (by ref)"))
  (bind (_bblockinghit _binitialoverlap _time _distance _location _impactpoint _normal _impactnormal _physmat _hitactor) (`GameplayStatics.BreakHitResult` Hit))
  (set `self.Seen Location` _location)
  (if (`self.ActorHasTag` _hitactor "Player")
    (`BlackboardComponent.SetValueAsBool` (`AIBlueprintHelperLibrary.GetBlackboard` (`AIBlueprintHelperLibrary.GetAIController` self)) "asSeenPlayer?" true)
    (bind _asbp_camera_controller (cast `/Game/Bp/Bp_CameraController` (`GameplayStatics.GetPlayerController` 0))
      (:`then`
        (`KismetSystemLibrary.PrintString` "Valid" true true (struct :`R` 0.148301 :`G` 1.0 :`A` 1.0))
        (`/Game/Bp/Bp_CameraController.DeathWidget` _asbp_camera_controller))
      (:`CastFailed`
        (`KismetSystemLibrary.PrintString` "Faild" true true (struct :`R` 1.0 :`G` 0.064825 :`A` 1.0))))
    (else
      (if (`BlackboardComponent.GetValueAsBool` (`AIBlueprintHelperLibrary.GetBlackboard` (`AIBlueprintHelperLibrary.GetAIController` self)) "asSeenPlayer?")
        (`KismetSystemLibrary.Delay` 5.0)
        (`|AIMoveTo` self (`self.Seen Location`) null
          (:`then`
            _)))
      (`BlackboardComponent.SetValueAsBool` (`AIBlueprintHelperLibrary.GetBlackboard` (`AIBlueprintHelperLibrary.GetAIController` self)) "asSeenPlayer?" false))))

(fn `UserConstructionScript`)