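; "Gordo" enemy character that patrols and detects the player by sight and hearing, reporting to Bp_V2AiController.
; Two line-traced mesh vision zones drive sight: the main reports the player with brief slow motion and spots dead enemies, the second sets a flag suppressing those player reports.
; AIPerception forwards heard noises to the controller.
; Also handles ragdoll death, outline toggling and a game-mode-driven highlight using a duplicate skeletal mesh.
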(event `Call Highlight`
  (params (NewParam :type Boolean))
  ;[0 1 0.0216] Begin Play
  (`self.Higlight` NewParam))

(event `self.ReceiveBeginPlay`
  (bind _zona_de_visao1 (`self.Zona De Visao1`))
  ;[0 1 0.0216] Begin Play
  (`|ExecutionSequence`
    (:`then_0`
      (`LineOfSightComponent.StartLineTrace` _zona_de_visao1 "TraceTypeQuery1" 120)
      (`LineOfSightComponent.StartLineTrace` (`self.Zona De Visao`) "TraceTypeQuery1" 120)
      (`LineOfSightComponent.StartBuildMesh` _zona_de_visao1)
      (`LineOfSightComponent.StartBuildMesh` (`self.Zona De Visao`))
      (`SceneComponent.SetHiddenInGame` (`self.Zona De Visao`) false false))
    (:`then_1`
      (bind _asmain_game_mode (cast `/Game/Bp/Main_GameMode` (`GameplayStatics.GetGameMode`)))
      (bind _output_get (set `self.As Main Game Mode` _asmain_game_mode))
      (add `/Game/Bp/Main_GameMode.HiglightSwitch` _output_get (delegate `Call Highlight`)))
    (:`then_2`
      (bind _asbp_v2ai_controller (cast `/Game/AI/Bp_V2AiController` (`self.GetController`)))
      (bind _output_get_2 (set `self.As Bp V2Ai Controller` _asbp_v2ai_controller))
      (set `/Game/AI/Bp_V2AiController.LookAroundPatrol` true _output_get_2))
    (:`then_3`
      (set `self.AnimationPatrolWalk` false)
      (set `self.Actor Dead?` false))
    (:`then_4`
      (`ActorComponent.Deactivate` (`self.DetectionInterrogatione`)))
    (:`then_5`
      (`BlackboardComponent.SetValueAsVector` (`AIController.Blackboard` (`self.As Bp V2Ai Controller`)) "PatrolLocations" (`self.K2_GetActorLocation`))
      (set `CharacterMovementComponent.MaxWalkSpeed` 300.0 (`self.CharacterMovement`)))))

(event `EnableOutline`
  (bind _mesh (`self.Mesh`))
  (bind _as_bp_v2ai_controller (`self.As Bp V2Ai Controller`))
  (if (`self.OutlineEnabled`)
    (`PrimitiveComponent.SetRenderCustomDepth` _mesh true)
    (set `self.OutlineEnabled` false)
    (set `/Game/AI/Bp_V2AiController.OutlineEnabled` true _as_bp_v2ai_controller)
    (else
      (`PrimitiveComponent.SetRenderCustomDepth` _mesh false)
      (set `self.OutlineEnabled` true)
      (set `/Game/AI/Bp_V2AiController.OutlineEnabled` true _as_bp_v2ai_controller))))

(event `Set Active FieldView`
  (bind _zona_de_visao (`self.Zona De Visao`))
  ;[0 0 0] Set Active FieldOfView
  (`SceneComponent.SetHiddenInGame` _zona_de_visao (not (`SceneComponent.bHiddenInGame` _zona_de_visao)) false)
  (`SceneComponent.SetHiddenInGame` (`self.Zona De Visao1`) (not (`SceneComponent.bHiddenInGame` _zona_de_visao)) false))

(event `/Game/Interfaces/RaggdollKill.Kill Actor`
  ;[0 0 0] Kill Actor
  (if (not (`self.Actor Dead?`))
    (set `/Game/AI/Bp_V2AiController.ActorDead` true (`self.As Bp V2Ai Controller`))
    (`CharacterMovementComponent.DisableMovement` (`self.CharacterMovement`))
    (`ActorComponent.K2_DestroyComponent` (`self.FMODAudio`))
    (`ActorComponent.K2_DestroyComponent` (`self.Zona De Visao`))
    (`ActorComponent.K2_DestroyComponent` (`self.Zona De Visao1`))
    (`PrimitiveComponent.SetSimulatePhysics` (`self.Mesh`) true)
    (`PrimitiveComponent.SetSimulatePhysics` (`self.Weapon`) true)
    (set `self.Actor Dead?` true)
    (`PrimitiveComponent.SetCollisionResponseToChannel` (`self.Mesh`) "ECC_GameTraceChannel2" "ECR_Ignore")))

(event `DestroiVisiom`
  ;[0 0 0] Destroi Line of Sight
  (`ActorComponent.K2_DestroyComponent` (`self.Zona De Visao`))
  (`ActorComponent.K2_DestroyComponent` (`self.Zona De Visao1`))
  (`CharacterMovementComponent.DisableMovement` (`self.CharacterMovement`)))

(event `PlaySound Death`
  ;[0 0 0] Play Sound Death
  (`FMODAudioComponent.Play` (`self.FMODAudio`)))

(event `self.Zona De Visao.BeginOverlap`
  (params (Hit :type "HitResult Structure (by ref)"))
  (bind (_bblockinghit _binitialoverlap _time _distance _location _impactpoint _normal _impactnormal _physmat _hitactor _hitcomponent) (`GameplayStatics.BreakHitResult` Hit))
  (bind _player (`/Game/Bp/Main_GameMode.Player` (`self.As Main Game Mode`)))
  (bind _returnvalue (`self.K2_GetActorLocation` _player))
  ;[0 0 0] FielOfView Overlap
  (set `self.Seen Location` _location)
  (if (`ActorComponent.ComponentHasTag` _hitcomponent "PlayerBody")
    (`GameplayStatics.SetGlobalTimeDilation` 0.3)
    (if (and (not (`self.EstaDentroZonaDeCharge`)) (not (`self.VisionInv`)))
      (`KismetSystemLibrary.PrintString` "Entrou" true true (struct :`R` 0.142881 :`G` 1.0 :`A` 1.0))
      (`/Game/AI/Bp_V2AiController.Recive Vision Of Player` (`self.As Bp V2Ai Controller`) _player _returnvalue)
      (`KismetSystemLibrary.DrawDebugBox` _returnvalue (40.0 40.0 100.0) (struct :`R` 1.0 :`G` 0.023343 :`A` 1.0) (struct) 100.0 10.0)
      (set `self.VisionInv` true)
      (`KismetSystemLibrary.K2_SetTimerDelegate` (delegate `Set VisionInv`) 0.5)
      (`KismetSystemLibrary.Delay` 0.2)
      (`GameplayStatics.SetGlobalTimeDilation` 1.0)
      (set `CharacterMovementComponent.MaxWalkSpeed` 500.0 (`self.CharacterMovement`)))
    (elif (`self.ActorHasTag` _hitactor "Enemy")
      (bind _asbp_v2ai_controller (cast `/Game/AI/Bp_V2AiController` (`AIBlueprintHelperLibrary.GetAIController` _hitactor)))
      (if (`/Game/AI/Bp_V2AiController.ActorDead` _asbp_v2ai_controller)
        (`/Game/AI/Bp_V2AiController.Viu Inimigo Morto` (`self.As Bp V2Ai Controller`) _hitactor)))))

(event `Set VisionInv`
  ;[0 0 0] FielOfView Overlap
  (set `self.VisionInv` false))

(event `self.Zona De Visao.EndOverlap`
  (params (Hit :type "HitResult Structure (by ref)"))
  ;[0 0 0] Sair Zona Verde
  (if (not (`self.EstaDentroZonaDeCharge`))
    (if (`ActorComponent.ComponentHasTag` (`.HitComponent` (`GameplayStatics.BreakHitResult` Hit)) "PlayerBody")
      (`LineOfSightComponent.StopInterpRadius` (`self.Zona De Visao1`))
      (`LineOfSightComponent.StopInterpRadius` (`self.Zona De Visao`))
      (`LineOfSightComponent.StopInterpRadius` (`self.Zona De Visao`))
      (`KismetSystemLibrary.PrintString` "Player Saiu" true true (struct :`R` 1.0 :`G` 0.076702 :`A` 1.0))
      (`/Game/AI/Bp_V2AiController.Recive EndOverlap` (`self.As Bp V2Ai Controller`)))))

(event `self.Zona De Visao1.BeginOverlap`
  (params (Hit :type "HitResult Structure (by ref)"))
  (bind (_bblockinghit _binitialoverlap _time _distance _location _impactpoint _normal _impactnormal _physmat _hitactor _hitcomponent) (`GameplayStatics.BreakHitResult` Hit))
  ;[0 0 0] Zona Amarela Begin Overlap
  (set `self.Seen Location` _location)
  (if (`ActorComponent.ComponentHasTag` _hitcomponent "PlayerBody")
    (set `self.EstaDentroZonaDeCharge` true)
    (`KismetSystemLibrary.Delay` 5.0)))

(event `self.AIPerception.OnTargetPerceptionUpdated`
  (params (Actor :type "Actor Object Reference") (Stimulus :type "AIStimulus Structure"))
  (bind (_age _expirationage _strength _stimuluslocation _receiverlocation _tag _bsuccessfullysensed) (break `AIStimulus` Stimulus))
  ;[0 0 0] Ouviu Algo
  (if _bsuccessfullysensed
    (bind _returnvalue (`AIPerceptionSystem.GetSenseClassForStimulus` Stimulus))
    (`KismetSystemLibrary.PrintString` "Sentiu algo")
    (if (== _returnvalue "/Script/AIModule.AISense_Hearing")
      (`/Game/AI/Bp_V2AiController.Ouviu Algo ` (`self.As Bp V2Ai Controller`) _stimuluslocation _tag))))

(event `Higlight`
  (params (Bool :type Boolean))
  (bind _mesh (`self.Mesh`))
  (`/Engine/EditorBlueprintResources/StandardMacros.IsValid` (`self.HiglightComp`)
    (:`Is Valid`
      (`SceneComponent.SetHiddenInGame` (`self.HiglightComp`) (not Bool) true))
    (:`Is Not Valid`
      (bind _returnvalue (`AddComponent|NODE_AddSkeletalMeshComponent-0` :`bManualAttachment` true :`RelativeTransform` (`SceneComponent.K2_GetComponentToWorld` _mesh)))
      (bind _output_get (set `self.HiglightComp` _returnvalue))
      (`SkeletalMeshComponent.SetSkeletalMeshAsset` _output_get (`SkeletalMeshComponent.GetSkeletalMeshAsset` (`self.Mesh`)))
      (`SkeletalMeshComponent.SetAnimInstanceClass` _output_get (`SkeletalMeshComponent.AnimClass` _mesh))
      (for (_ _array_index) (`MeshComponent.GetMaterials` (`self.HiglightComp`))
        (`PrimitiveComponent.SetMaterial` (`self.HiglightComp`) _array_index "/Game/mate/M_OutLine_InstINIMIGO.M_OutLine_InstINIMIGO")))))

(fn `Fake End OVerlap`
  (params (Hit :type "HitResult Structure")))

(fn `Fake Overlap 2`
  (params (Hit :type "HitResult Structure")))

(fn `FakeBegin Overlap`
  (params (Hit :type "HitResult Structure (by ref)")))

(fn `UserConstructionScript`)