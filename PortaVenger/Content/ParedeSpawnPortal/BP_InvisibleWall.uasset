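; Invisible wall that opens a Niagara portal where it is clicked, at a set height and clamped within the wall's edges.
; BeginPlay uses actor yaw and component bounds to find two inset endpoints along X or Y, drawn as debug shapes.
; SpawnPortal uses the click normal to pick the clamping axis.
; It then spawns the portal, an aim point, a portal arm told to HandGrab it, and a second portal beside the player.
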(event `self.ReceiveBeginPlay`
  (bind _origin (`self.Origin`))
  (bind _origin_2 (`self.Origin`))
  (bind _x (.x (`self.MaxXPointWall`)))
  (bind _y (.y (`self.MaxXPointWall`)))
  (bind _z (.z (`self.MaxXPointWall`)))
  (bind _x_2 (.x (`self.MinXPointWall`)))
  (bind _y_2 (.y (`self.MinXPointWall`)))
  (bind _z_2 (.z (`self.MinXPointWall`)))
  (bind _x_3 (.x (`self.MaxXPointWall`)))
  (bind _y_3 (.y (`self.MaxXPointWall`)))
  (bind _z_3 (.z (`self.MaxXPointWall`)))
  (bind _x_4 (.x (`self.MinXPointWall`)))
  (bind _y_4 (.y (`self.MinXPointWall`)))
  (bind _z_4 (.z (`self.MinXPointWall`)))
  (bind _returnvalue (`self.GetTransform` self))
  (bind (_origin_3 _boxextent) (`KismetSystemLibrary.GetComponentBounds` (`self.d`)))
  (set `self.Origin` _origin_3)
  (set `self.Box Extent` _boxextent)
  (if (or (`KismetMathLibrary.NearlyEqual_FloatFloat` (.yaw (.rotation _returnvalue)) -90.0 0.1) (`KismetMathLibrary.NearlyEqual_FloatFloat` (.yaw (.rotation _returnvalue)) 90.0 0.1))
    ;[1 1 1] Set Values
    (bind _output_get (set `self.MaxXPointWall` (`KismetMathLibrary.MakeVector` (.x (+ _origin (`KismetMathLibrary.MakeVector` (- (.x (`self.Box Extent`)) 100.0)))) (.y (+ _origin (`KismetMathLibrary.MakeVector` (- (.x (`self.Box Extent`)) 100.0)))) (`self.SetPortalHeight`))))
    (bind _output_get_2 (set `self.MinXPointWall` (`KismetMathLibrary.MakeVector` (.x (- _origin (`KismetMathLibrary.MakeVector` (- (.x (`self.Box Extent`)) 100.0)))) (.y (- _origin (`KismetMathLibrary.MakeVector` (- (.x (`self.Box Extent`)) 100.0)))) (`self.SetPortalHeight`))))
    (`KismetSystemLibrary.DrawDebugBox` _output_get (10.0 10.0 10.0) (struct :`R` 1.0 :`G` 0.093821 :`A` 1.0) (struct) 10000.0)
    (`KismetSystemLibrary.DrawDebugBox` _output_get_2 (10.0 10.0 10.0) (struct :`G` 1.0 :`B` 0.040351 :`A` 1.0) (struct) 10000.0)
    (`KismetSystemLibrary.DrawDebugLine` (`self.MaxXPointWall`) (`self.MinXPointWall`) (struct :`G` 1.0 :`B` 0.080067 :`A` 1.0) 1000.0 10.0)
    (`KismetSystemLibrary.DrawDebugLine` (`KismetMathLibrary.MakeVector` _x_3 _y_3 (- _z_3 (`self.SetPortalHeight`))) (`KismetMathLibrary.MakeVector` _x_3 _y_3 (+ _z_3 1000.0)) (struct :`R` 1.0 :`G` 0.089371 :`A` 1.0) 1000.0 10.0)
    (`KismetSystemLibrary.DrawDebugLine` (`KismetMathLibrary.MakeVector` _x_4 _y_4 (- _z_4 (`self.SetPortalHeight`))) (`KismetMathLibrary.MakeVector` _x_4 _y_4 (+ _z_4 1000.0)) (struct :`R` 1.0 :`G` 0.089371 :`A` 1.0) 1000.0 10.0)
    (else
      ;[1 1 1] Set Value
      (bind _output_get_3 (set `self.MaxXPointWall` (`KismetMathLibrary.MakeVector` (.x (+ _origin_2 (`KismetMathLibrary.MakeVector` 0.0 (- (.y (`self.Box Extent`)) 100.0) (* (`self.SetPortalHeight`) -1.0)))) (.y (+ _origin_2 (`KismetMathLibrary.MakeVector` 0.0 (- (.y (`self.Box Extent`)) 100.0) (* (`self.SetPortalHeight`) -1.0)))) (`self.SetPortalHeight`))))
      (bind _output_get_4 (set `self.MinXPointWall` (`KismetMathLibrary.MakeVector` (.x (- _origin_2 (`KismetMathLibrary.MakeVector` 0.0 (- (.y (`self.Box Extent`)) 100.0) (`self.SetPortalHeight`)))) (.y (- _origin_2 (`KismetMathLibrary.MakeVector` 0.0 (- (.y (`self.Box Extent`)) 100.0) (`self.SetPortalHeight`)))) (`self.SetPortalHeight`))))
      (`KismetSystemLibrary.DrawDebugBox` _output_get_3 (10.0 10.0 10.0) (struct :`R` 1.0 :`G` 0.093821 :`A` 1.0) (struct) 10000.0)
      (`KismetSystemLibrary.DrawDebugBox` _output_get_4 (10.0 10.0 10.0) (struct :`G` 1.0 :`B` 0.040351 :`A` 1.0) (struct) 10000.0)
      (`KismetSystemLibrary.DrawDebugLine` (`self.MaxXPointWall`) (`self.MinXPointWall`) (struct :`G` 1.0 :`B` 0.080067 :`A` 1.0) 1000.0 10.0)
      (`KismetSystemLibrary.DrawDebugLine` (`KismetMathLibrary.MakeVector` _x _y (- _z (`self.SetPortalHeight`))) (`KismetMathLibrary.MakeVector` _x _y (+ _z 1000.0)) (struct :`R` 1.0 :`G` 0.089371 :`A` 1.0) 1000.0 10.0)
      (`KismetSystemLibrary.DrawDebugLine` (`KismetMathLibrary.MakeVector` _x_2 _y_2 (- _z_2 (`self.SetPortalHeight`))) (`KismetMathLibrary.MakeVector` _x_2 _y_2 (+ _z_2 1000.0)) (struct :`R` 1.0 :`G` 0.089371 :`A` 1.0) 1000.0 10.0))))

(event `/Game/Interfaces/SpawnPortal.SpawnPortal`
  (params (ClickLocation :type "Vector Structure") (NormalClickLocation :type "Vector Structure") (X1 :type "/Game/Bp/Bp_Character Object Reference"))
  ;[1 1 1] Quando clica na parede acontece
  (`|ExecutionSequence`
    (:`then_0`
      (`/Engine/EditorBlueprintResources/StandardMacros.DoOnce` false
        (:`Completed`
          (set `self.X1` X1))))
    (:`then_1`
      (set `self.Click Location` ClickLocation)
      (set `self.Normal Click Location` NormalClickLocation)
      (`self.Set ClickPoint To the Correct Z axis`)
      (`self.Calc Wall direction`))))

(event `Spawn NiagaraPortal`
  (params (Position :type "Vector Structure"))
  (bind _returnvalue (`self.GetTransform` (`self.X1`)))
  ;[1 1 1] Portal da parede
  (bind _returnvalue_2 (`NiagaraFunctionLibrary.SpawnSystemAtLocation` "/Game/StarterContent/Maps/CaixaDeAreiaVFXs/Portal/NS_Portal3.NS_Portal3" Position (* (`self.K2_GetActorRotation` self) -1.0)))
  (bind (_returnvalue_roll _returnvalue_pitch _returnvalue_yaw) (`KismetMathLibrary.BreakRotator` (`SceneComponent.K2_GetComponentRotation` _returnvalue_2)))
  (bind _returnvalue_3 (`KismetMathLibrary.MakeTransform` (`SceneComponent.K2_GetComponentLocation` _returnvalue_2) (`KismetMathLibrary.MakeRotator` _returnvalue_roll 0.0 _returnvalue_yaw)))
  (bind _returnvalue_4 (`|SpawnActorFromClass` "/Game/Bp/Bp_AimPoint.Bp_AimPoint_C" _returnvalue_3 "Undefined" "MultiplyWithRoot" null null))
  (bind _returnvalue_5 (`|SpawnActorFromClass` "/Game/Bp/Bp_PortalArm.Bp_PortalArm_C" _returnvalue_3 "AlwaysSpawn" "MultiplyWithRoot" null null))
  (`/Game/Bp/Bp_PortalArm.HandGrab` _returnvalue_5 _returnvalue_4)
  ;[1 1 1] Portal do player
  (`NiagaraFunctionLibrary.SpawnSystemAtLocation` "/Game/StarterContent/Maps/CaixaDeAreiaVFXs/Portal/NS_Portal3.NS_Portal3" (`KismetMathLibrary.MakeVector` (+ (.x (.location _returnvalue)) 150.0) (+ (.y (.location _returnvalue)) 150.0) (- (.z (.location _returnvalue)) 100.0)) (`KismetMathLibrary.MakeRotator` (.roll (.rotation _returnvalue)) 90.0 (.yaw (.rotation _returnvalue)))))

(event `Calc Wall direction`
  (bind _normal_click_location (`self.Normal Click Location`))
  (if (or (== _normal_click_location (1.0 0.0 0.0) :`ErrorTolerance` 0.1) (== _normal_click_location (-1.0 0.0 0.0) :`ErrorTolerance` 0.1))
    ;[1 1 1] True a direita
    (if (> (.y (`self.Origin`)) (.y (`self.Click Location`)))
      (if (> (.y (`self.Click Location`)) (.y (`self.MinXPointWall`)))
        (`KismetSystemLibrary.PrintString` "Nao Passou")
        (`self.Spawn NiagaraPortal` (`self.Click Location`))
        (else
          (`KismetSystemLibrary.PrintString` "Passou")
          (`self.Spawn NiagaraPortal` (`self.MinXPointWall`))))
      (else
        ;[1 1 1] Se passa do bound
        (if (< (.y (`self.Click Location`)) (.y (`self.MaxXPointWall`)))
          (`KismetSystemLibrary.PrintString` "Nao Passou")
          (`self.Spawn NiagaraPortal` (`self.Click Location`))
          (else
            ;[1 1 1] Caso passe spawnar no ponto certo
            (`KismetSystemLibrary.PrintString` "Passou")
            (`self.Spawn NiagaraPortal` (`self.MaxXPointWall`))))))
    (elif (> (.x (`self.Origin`)) (.x (`self.Click Location`)))
      (if (> (.x (`self.Click Location`)) (.x (`self.MinXPointWall`)))
        (`KismetSystemLibrary.PrintString` "Nao Passou")
        (`self.Spawn NiagaraPortal` (`self.Click Location`))
        (else
          (`KismetSystemLibrary.PrintString` "Passou")
          (`self.Spawn NiagaraPortal` (`self.MinXPointWall`))))
      (else
        ;[1 1 1] Se passa do bound
        (if (< (.x (`self.Click Location`)) (.x (`self.MaxXPointWall`)))
          (`KismetSystemLibrary.PrintString` "Nao Passou")
          (`self.Spawn NiagaraPortal` (`self.Click Location`))
          (else
            ;[1 1 1] Caso passe spawnar no ponto certo
            (`KismetSystemLibrary.PrintString` "Passou")
            (`self.Spawn NiagaraPortal` (`self.MaxXPointWall`))))))))

(event `Set ClickPoint To the Correct Z axis`
  ;[1 1 1] Colocar o click location com a altura certa
  (set `self.Click Location` (`KismetMathLibrary.MakeVector` (.x (`self.Click Location`)) (.y (`self.Click Location`)) (`self.SetPortalHeight`))))

(fn `UserConstructionScript`)